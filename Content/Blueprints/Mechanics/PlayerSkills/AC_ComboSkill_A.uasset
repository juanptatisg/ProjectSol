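; AC_ComboSkill_A is a multi-hit player combo skill that spends energy to damage and stagger an enemy.
; StartSkill checks energy, playing a sound if short, otherwise locks the player into the skill flipbook and updates the energy bar.
; A delay-driven loop raises the combo counter by two per hit and deals damage scaled by Attack, Level, variance and crit chance, which also boosts stagger.
; After the last hit, endlag restores idle and clears the locks.
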(event EventStartSkill
  (params (player :type BP%20Player%20Battler%20Object%20Reference) (enemy :type BP%20Enemy%20Base%20Object%20Reference))
  (bind _basedamage (Variables|Default|GetBaseDamage))
  (if (>= (Variables|/Game/Blueprints/BP_PlayerBattler.BP_PlayerBattler_C|GetCurrentEnergy player) (Variables|Default|GetCost))
    (bind _output_get (Variables|Default|SetPlayerRef player))
    (Variables|Default|SetEnemyRef enemy)
    (Variables|/Game/Blueprints/BP_PlayerBattler.BP_PlayerBattler_C|SetInAnimation _output_get true)
    (Variables|/Game/Blueprints/BP_PlayerBattler.BP_PlayerBattler_C|SetSkillCD _output_get true)
    ;[1 1 1] Skill-specific FB (might need rework on Combo Skills)
    (Sprite|SetFlipbook (Variables|/Game/Blueprints/BP_PlayerBattler.BP_PlayerBattler_C|GetPaperFlipbook _output_get) (Variables|Default|GetSkillAnimation))
    ;[0 1 1] Energy Cost Reduction
    (Variables|/Game/Blueprints/BP_PlayerBattler.BP_PlayerBattler_C|SetOldEnergy (Variables|Default|GetPlayerRef) (Variables|/Game/Blueprints/BP_PlayerBattler.BP_PlayerBattler_C|GetCurrentEnergy (Variables|Default|GetPlayerRef)))
    (Variables|/Game/Blueprints/BP_PlayerBattler.BP_PlayerBattler_C|SetCurrentEnergy (Variables|Default|GetPlayerRef) (- (Variables|/Game/Blueprints/BP_PlayerBattler.BP_PlayerBattler_C|GetCurrentEnergy (Variables|Default|GetPlayerRef)) (Variables|Default|GetCost)))
    (Default|ChangeBarEnergy (Variables|Default|GetPlayerRef))
    (Variables|Default|SetHitsCounter 1)
    ;[0 1 0] Skill Startup Lag
    (Utilities|FlowControl|Delay (Variables|Default|GetSkillDuration) :!label _label)
    ;[1 1 1] Combo Increment
    (Math|Integer|IncrementInt (Variables|/Game/Blueprints/BP_PlayerBattler.BP_PlayerBattler_C|GetComboCounter (Variables|Default|GetPlayerRef))
      (:%20%20
        (Math|Integer|IncrementInt (Variables|/Game/Blueprints/BP_PlayerBattler.BP_PlayerBattler_C|GetComboCounter (Variables|Default|GetPlayerRef))
          (:%20%20
            (Utilities|FlowControl|Sequence
              (:then_0
                (Default|TakeDamageEnemy (Variables|Default|GetEnemyRef) (+ (* (* (+ (+ _basedamage (* (/ _basedamage 1e+01) (.attack (Variables|/Game/Blueprints/BP_PlayerBattler.BP_PlayerBattler_C|GetStatsMod (Variables|Default|GetPlayerRef))))) (* (.level (Variables|/Game/Blueprints/BP_PlayerBattler.BP_PlayerBattler_C|GetStatsMod (Variables|Default|GetPlayerRef))) 2)) (Math|Random|RandomFloatinRange 0.9 1.0)) (Math|Float|SelectFloat 1.0 1.25 (>= (Math|Random|RandomIntegerinRange 1 100) (* (.critrate (Variables|/Game/Blueprints/BP_PlayerBattler.BP_PlayerBattler_C|GetStatsMod (Variables|Default|GetPlayerRef))) 1e+02)))) 1.0) (Variables|Default|GetStaggerDamage) (Math|Float|SelectFloat 1.0 2.0 (>= (Math|Random|RandomIntegerinRange 1 100) (* (.critrate (Variables|/Game/Blueprints/BP_PlayerBattler.BP_PlayerBattler_C|GetStatsMod (Variables|Default|GetPlayerRef))) 1e+02))))
                (Default|ChangeBarEnemy (Variables|Default|GetEnemyRef)))
              (:then_1
                (if (<= (Variables|Default|GetNumberOfHits) (Variables|Default|GetHitsCounter))
                  ;[0 1 0] Animation Endlag
                  (Utilities|FlowControl|Delay (Variables|Default|GetEndlag))
                  ;[1 1 1] Idle Battle FB
                  (Sprite|SetFlipbook (Variables|/Game/Blueprints/BP_PlayerBattler.BP_PlayerBattler_C|GetPaperFlipbook (Variables|Default|GetPlayerRef)) "/Game/Assets/Scum/Flipbooks/FB_PlayerIdle.FB_PlayerIdle")
                  (Variables|/Game/Blueprints/BP_PlayerBattler.BP_PlayerBattler_C|SetInAnimation (Variables|Default|GetPlayerRef) false)
                  (Variables|/Game/Blueprints/BP_PlayerBattler.BP_PlayerBattler_C|SetSkillCD (Variables|Default|GetPlayerRef) false)
                  (else
                    (Math|Integer|IncrementInt (Variables|Default|GetHitsCounter)
                      (:%20%20
                        (goto _label)))))))))))
    (else
      (Audio|PlaySound2D "/Game/Assets/Audio/SFX/HitNoise.HitNoise" 2.0 1.0 0.0 "/Game/Assets/Audio/SC_BattleEffects.SC_BattleEffects" 0))))