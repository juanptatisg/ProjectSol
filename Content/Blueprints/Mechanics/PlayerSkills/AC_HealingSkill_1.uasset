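; Player skill component for a turn-based or battle-style healing ability that spends energy to restore the player's health.
; StartSkill checks energy, sets animation and cooldown flags, plays the skill flipbook and deducts the cost, or plays a sound if energy is short.
; After a startup delay it heals from max HP percentage plus Healing stat, with random variance and crit multiplier.
; An endlag delay then restores the idle flipbook and clears both flags.
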(event EventStartSkill
  (params (player :type BP%20Player%20Battler%20Object%20Reference) (enemy :type BP%20Enemy%20Base%20Object%20Reference))
  (if (>= (Variables|/Game/Blueprints/BP_PlayerBattler.BP_PlayerBattler_C|GetCurrentEnergy player) (Variables|Default|GetCost))
    (bind _output_get (Variables|Default|SetPlayerRef player))
    (Variables|Default|SetEnemyRef enemy)
    (Variables|/Game/Blueprints/BP_PlayerBattler.BP_PlayerBattler_C|SetInAnimation _output_get true)
    (Variables|/Game/Blueprints/BP_PlayerBattler.BP_PlayerBattler_C|SetSkillCD _output_get true)
    ;[1 1 1] Skill-specific FB
    (Sprite|SetFlipbook (Variables|/Game/Blueprints/BP_PlayerBattler.BP_PlayerBattler_C|GetPaperFlipbook _output_get) (Variables|Default|GetSkillAnimation))
    ;[0 1 1] Energy Cost Reduction
    (Variables|/Game/Blueprints/BP_PlayerBattler.BP_PlayerBattler_C|SetOldEnergy (Variables|Default|GetPlayerRef) (Variables|/Game/Blueprints/BP_PlayerBattler.BP_PlayerBattler_C|GetCurrentEnergy (Variables|Default|GetPlayerRef)))
    (Variables|/Game/Blueprints/BP_PlayerBattler.BP_PlayerBattler_C|SetCurrentEnergy (Variables|Default|GetPlayerRef) (- (Variables|/Game/Blueprints/BP_PlayerBattler.BP_PlayerBattler_C|GetCurrentEnergy (Variables|Default|GetPlayerRef)) (Variables|Default|GetCost)))
    (Default|ChangeBarEnergy (Variables|Default|GetPlayerRef))
    ;[0 1 0] Skill Startup Lag
    (Utilities|FlowControl|Delay (Variables|Default|GetStartup))
    (Default|GainHealth (Variables|Default|GetPlayerRef) (Math|Conversions|ToFloat(Integer) (Math|Float|Round (* (* (+ (* (.MaxHP (Utilities|Struct|BreakST_Stats (Variables|/Game/Blueprints/BP_PlayerBattler.BP_PlayerBattler_C|GetStatsMod (Variables|Default|GetPlayerRef)))) (/ (Variables|Default|GetBaseHealing) 1e+02)) (.healing (Variables|/Game/Blueprints/BP_PlayerBattler.BP_PlayerBattler_C|GetStatsMod (Variables|Default|GetPlayerRef)))) (Math|Random|RandomFloatinRange 0.9 1.0)) (Math|Float|SelectFloat 1.0 1.5 (>= (Math|Random|RandomIntegerinRange 1 100) (* (.critrate (Variables|/Game/Blueprints/BP_PlayerBattler.BP_PlayerBattler_C|GetStatsMod (Variables|Default|GetPlayerRef))) 1e+02)))))))
    (Default|ChangeBarHealth (Variables|Default|GetPlayerRef))
    ;[0 1 0] Animation Endlag
    (Utilities|FlowControl|Delay (Variables|Default|GetEndlag))
    ;[1 1 1] Idle Battle FB
    (Sprite|SetFlipbook (Variables|/Game/Blueprints/BP_PlayerBattler.BP_PlayerBattler_C|GetPaperFlipbook (Variables|Default|GetPlayerRef)) "/Game/Assets/Scum/Flipbooks/FB_PlayerIdle.FB_PlayerIdle")
    (Variables|/Game/Blueprints/BP_PlayerBattler.BP_PlayerBattler_C|SetInAnimation (Variables|Default|GetPlayerRef) false)
    (Variables|/Game/Blueprints/BP_PlayerBattler.BP_PlayerBattler_C|SetSkillCD (Variables|Default|GetPlayerRef) false)
    (else
      (Audio|PlaySound2D "/Game/Assets/Audio/SFX/HitNoise.HitNoise" 2.0 1.0 0.0 "/Game/Assets/Audio/SC_BattleEffects.SC_BattleEffects" 0))))