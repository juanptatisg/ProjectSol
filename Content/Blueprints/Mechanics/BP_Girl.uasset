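; BP_Girl is a 2D Paper2D girl character that displays a flipbook animation matching her current animation state.
; On BeginPlay it calls UpdateFlipbook, which switches on the AnimationState enum.
; Each state (idle, sitting, unconscious or scarf) sets its own flipbook on the PaperFlipbook component.
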(event EventBeginPlay
  (CallFunction|UpdateFlipbook))

(fn ConstructionScript)

(fn UpdateFlipbook
  (switch Utilities|FlowControl|Switch|SwitchonENM_GirlStates (Variables|Default|GetAnimationState)
    (:NewEnumerator0
      (Sprite|SetFlipbook (Variables|Default|GetPaperFlipbook) (Variables|Default|GetFBIdle)))
    (:NewEnumerator1
      (Sprite|SetFlipbook (Variables|Default|GetPaperFlipbook) (Variables|Default|GetFBSit)))
    (:NewEnumerator3
      (Sprite|SetFlipbook (Variables|Default|GetPaperFlipbook) (Variables|Default|GetFBRest)))
    (:NewEnumerator4
      (Sprite|SetFlipbook (Variables|Default|GetPaperFlipbook) (Variables|Default|GetFBScarf)))))