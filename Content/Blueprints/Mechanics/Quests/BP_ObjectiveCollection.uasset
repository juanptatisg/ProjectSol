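; Composite quest objective that groups sub-objectives and finishes once all of them are complete.
; On activation it either starts the sub-objectives one after another when Ordered, or all at once otherwise.
; Finish events from sub-objectives drive the sequence or completion check, and their updates are forwarded as the collection's own update.
; Completion progress is the equally weighted average of the sub-objectives' progress, so collections can report like single objectives.
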(event Custom|ForwardUpdateObjective
  (params (Objective :type BP%20Base%20Objective%20Object%20Reference))
  (Default|CallUpdateObjective self))

(event Custom|OnObjectiveFinished
  (params (Objective :type BP%20Base%20Objective%20Object%20Reference))
  (CallFunction|FCheckObjectiveCollectionFinished)
  (EventDispatchers|UnbindEventfromFinishObjective Objective (delegate Custom|OnObjectiveFinished))
  (Default|CallUpdateObjective self))

(event Custom|On%20ObjectiveSequenceCompleted
  (params (Objective :type BP%20Base%20Objective%20Object%20Reference))
  (EventDispatchers|UnbindEventfromFinishObjective Objective (delegate Custom|On%20ObjectiveSequenceCompleted))
  (CallFunction|FActivateNextObjective (delegate Custom|On%20ObjectiveSequenceCompleted))
  (Default|CallUpdateObjective self))

(event EventFActivateObjective
  (|CallParentFunction)
  (for _array_element (Variables|Default|GetSubObjectives)
    (EventDispatchers|BindEventtoUpdateObjective _array_element (delegate Custom|ForwardUpdateObjective)))
  (if (Variables|Default|GetOrdered)
    (CallFunction|FActivateNextObjective (delegate Custom|On%20ObjectiveSequenceCompleted))
    (else
      (for _array_element_2 (Variables|Default|GetSubObjectives)
        (Default|FActivateObjective _array_element_2)
        (EventDispatchers|BindEventtoFinishObjective _array_element_2 (delegate Custom|OnObjectiveFinished)))))
  (Default|CallUpdateObjective self))

(fn FCheckObjectiveCollectionFinished
  (for _array_element (Variables|Default|GetSubObjectives)
    (if (not (Variables|/Game/Blueprints/Mechanics/Quests/BP_BaseObjective.BP_BaseObjective_C|GetIsComplete _array_element))
      (return)))
  (CallFunction|FFinishObjective))

(fn FActivateNextObjective
  (params (Event :type Delegate%20%28by%20ref%29))
  (for _array_element (Variables|Default|GetSubObjectives)
    (if (not (Variables|/Game/Blueprints/Mechanics/Quests/BP_BaseObjective.BP_BaseObjective_C|GetIsActive _array_element))
      (Default|FActivateObjective _array_element)
      (EventDispatchers|BindEventtoFinishObjective _array_element Event)
      (return)))
  (CallFunction|FCheckObjectiveCollectionFinished))

(fn FGetCompletionProgress
  (for _array_element 0
    (bind _completionrate (CallFunction|FGetCompletionProgress _array_element))
    (LocalVariables|SetCompleteRate (+ (LocalVariables|GetCompleteRate) (/ _completionrate (Math|Conversions|ToFloat(Integer) (Utilities|Array|Length (Variables|Default|GetSubObjectives)))))))
  (return (LocalVariables|GetCompleteRate)))