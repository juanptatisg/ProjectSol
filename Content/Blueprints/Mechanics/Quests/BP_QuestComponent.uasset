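; A quest component that tracks active and finished quests in maps keyed by quest ID.
; Adding a quest skips known ones, stores it as active, binds its update and completion events, and starts it.
; Completion moves a quest to the finished map, and both completion and the UI update function refresh the quest list widget.
; Tick iterates both maps' keys with empty loop bodies.
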(event EventTick
  (params (DeltaSeconds :type Float%20%28single-precision%29))
  (bind _keys (Utilities|Map|Keys (Variables|Default|GetActiveQuests)))
  (for _array_element _keys
    _)
  (bind _keys_2 (Utilities|Map|Keys (Variables|Default|GetFinishedQuests)))
  (for _array_element_2 _keys_2
    _))

(fn FIsQuestActive
  (params (QuestToCheck :type BP%20Base%20Quest%20Object%20Reference))
  (return (Utilities|Map|Contains (Variables|Default|GetActiveQuests) (Variables|/Game/Blueprints/Mechanics/Quests/BP_BaseQuest.BP_BaseQuest_C|GetQuestID QuestToCheck))))

(fn FIsQuestFinished
  (params (QuestToCheck :type BP%20Base%20Quest%20Object%20Reference))
  (return (Utilities|Map|Contains (Variables|Default|GetFinishedQuests) (Variables|/Game/Blueprints/Mechanics/Quests/BP_BaseQuest.BP_BaseQuest_C|GetQuestID QuestToCheck))))

(fn FAddQuest
  (params (QuestToAdd :type BP%20Base%20Quest%20Object%20Reference))
  (if (and (not (CallFunction|FIsQuestActive QuestToAdd)) (not (CallFunction|FIsQuestFinished QuestToAdd)))
    (Utilities|Map|Add (Variables|Default|GetActiveQuests) (Variables|/Game/Blueprints/Mechanics/Quests/BP_BaseQuest.BP_BaseQuest_C|GetQuestID QuestToAdd) QuestToAdd)
    (EventDispatchers|BindEventtoQuestUpdated QuestToAdd (EventDispatchers|CreateEvent :!event FUpdateUI))
    (Default|StartQuest QuestToAdd)
    (EventDispatchers|BindEventtoCompletedQuest QuestToAdd (EventDispatchers|CreateEvent :!event FCompleteQuest))
    (Default|CallQuestUpdated QuestToAdd)))

(fn FCompleteQuest
  (params (CompletedQuest :type BP%20Base%20Quest%20Object%20Reference))
  (bind _questid (Variables|/Game/Blueprints/Mechanics/Quests/BP_BaseQuest.BP_BaseQuest_C|GetQuestID CompletedQuest))
  (Utilities|Map|Remove (Variables|Default|GetActiveQuests) _questid)
  (Utilities|Map|Add (Variables|Default|GetFinishedQuests) _questid CompletedQuest)
  (Default|UpdateQuestList (Variables|Default|GetQuestUI)))

(fn FUpdateUI
  (Default|UpdateQuestList (Variables|Default|GetQuestUI)))