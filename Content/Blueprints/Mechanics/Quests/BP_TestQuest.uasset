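; BP_TestQuest is a test quest that sends the player to three places: Location1, a village and Lucia's Tree.
; InitObjectives builds a location objective for each, binding a location trigger, display name and ID.
; It wraps them as sub-objectives in a BP_ObjectiveCollection and returns that collection.
; The event graph is disabled and the construction script only calls its parent, so this asset only defines objectives.
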(event EventBeginPlay
  (|CallParentFunction) ; This node is disabled and will not be called.\nDrag off pins to build functionality.
)

(event Collision|EventActorBeginOverlap
  (params (OtherActor :type Actor%20Object%20Reference))
  (|CallParentFunction OtherActor) ; This node is disabled and will not be called.\nDrag off pins to build functionality.
)

(event EventTick
  (params (DeltaSeconds :type Float%20%28single-precision%29))
  (|CallParentFunction DeltaSeconds) ; This node is disabled and will not be called.\nDrag off pins to build functionality.
)

(fn ConstructionScript
  (|CallParentFunction))

(fn InitObjectives
  (bind _returnvalue (Game|ConstructObjectfromClass "/Game/Blueprints/Mechanics/Quests/BP_LocationObjective.BP_LocationObjective_C" (Variables|Default|GetLocation1) "EnterLocation1" "LocationTrigger1"))
  (bind _returnvalue_2 (Game|ConstructObjectfromClass "/Game/Blueprints/Mechanics/Quests/BP_LocationObjective.BP_LocationObjective_C" (Variables|Default|GetLocation2) "EnterVillage" "LocationTrigger2"))
  (bind _returnvalue_3 (Game|ConstructObjectfromClass "/Game/Blueprints/Mechanics/Quests/BP_LocationObjective.BP_LocationObjective_C" (Variables|Default|GetLocation3) "EnterLucia's Tree" "LocationTrigger3"))
  (bind _returnvalue_4 (Game|ConstructObjectfromClass "/Game/Blueprints/Mechanics/Quests/BP_ObjectiveCollection.BP_ObjectiveCollection_C" (Utilities|Array|MakeArray _returnvalue _returnvalue_2 _returnvalue_3)))
  (return _returnvalue_4))