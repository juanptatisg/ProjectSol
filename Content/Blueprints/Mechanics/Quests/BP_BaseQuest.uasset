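; Base quest Blueprint that runs a root objective with sub-objectives and reports quest progress and completion.
; StartQuest gets the root objective from InitObjectives, whose base version only prints a debug message and is apparently meant to be overridden, then activates it.
; It binds root completion to CallCompletedQuest, while root updates and direct sub-objective updates or completions feed CallQuestUpdated, which also fires once at start.
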(event Custom|OnQuestCompleted
  (params (Objective :type BP%20Base%20Objective%20Object%20Reference))
  (Default|CallCompletedQuest self))

(event Custom|StartQuest
  (bind _objectives (CallFunction|InitObjectives))
  (bind _output_get (Variables|Default|SetObjectives _objectives))
  (Default|FActivateObjective _output_get)
  (EventDispatchers|BindEventtoFinishObjective _output_get (delegate Custom|OnQuestCompleted))
  (EventDispatchers|BindEventtoUpdateObjective _output_get (delegate Custom|OnQuestUpdated))
  (for _array_element (Variables|/Game/Blueprints/Mechanics/Quests/BP_ObjectiveCollection.BP_ObjectiveCollection_C|GetSubObjectives (Variables|Default|GetObjectives))
    (EventDispatchers|BindEventtoUpdateObjective _array_element (delegate Custom|UpdateObjectiveEvent))
    (EventDispatchers|BindEventtoFinishObjective _array_element (delegate Custom|UpdateObjectiveEvent)))
  (Default|CallQuestUpdated))

(event Custom|OnQuestUpdated
  (params (Objective :type BP%20Base%20Objective%20Object%20Reference))
  (Default|CallQuestUpdated self))

(event Custom|UpdateObjectiveEvent
  (params (Objective :type BP%20Base%20Objective%20Object%20Reference))
  (Default|CallQuestUpdated))

(fn ConstructionScript)

(fn InitObjectives
  (Development|PrintString "PARENT OBJECTIVER INIT CALLED" true true "(R=1.000000,G=0.000000,B=0.015782,A=1.000000)")
  (return 0))