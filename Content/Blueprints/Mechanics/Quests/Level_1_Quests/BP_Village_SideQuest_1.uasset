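; Village side quest for Level 1 that tasks the player with killing ten Forest Sprites.
; InitObjectives constructs one BP_EnemyKillObjective per referenced sprite and returns them wrapped in a BP_ObjectiveCollection named "Kill Forest Sprites".
; The collection is flagged Ordered, with its sub-objectives listed as sprite 1 first, then 10 down to 2.
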(fn InitObjectives
  (bind _returnvalue (Game|ConstructObjectfromClass "/Game/Blueprints/Mechanics/Quests/BP_EnemyKillObjective.BP_EnemyKillObjective_C" (Variables|Default|GetForestSprite1) "Kill Forest Sprite1" "Kill Forest Sprite1"))
  (bind _returnvalue_2 (Game|ConstructObjectfromClass "/Game/Blueprints/Mechanics/Quests/BP_EnemyKillObjective.BP_EnemyKillObjective_C" (Variables|Default|GetForestSprite2) "Kill Forest Sprite 2" "Kill Forest Sprite 2"))
  (bind _returnvalue_3 (Game|ConstructObjectfromClass "/Game/Blueprints/Mechanics/Quests/BP_EnemyKillObjective.BP_EnemyKillObjective_C" (Variables|Default|GetForestSprite3) "Kill Forest Sprite 3" "Kill Forest Sprite 3"))
  (bind _returnvalue_4 (Game|ConstructObjectfromClass "/Game/Blueprints/Mechanics/Quests/BP_EnemyKillObjective.BP_EnemyKillObjective_C" (Variables|Default|GetForestSprite4) "Kill Forest Sprite 4" "Kill Forest Sprite 4"))
  (bind _returnvalue_5 (Game|ConstructObjectfromClass "/Game/Blueprints/Mechanics/Quests/BP_EnemyKillObjective.BP_EnemyKillObjective_C" (Variables|Default|GetForestSprite5) "Kill Forest Sprite 5" "Kill Forest Sprite 5"))
  (bind _returnvalue_6 (Game|ConstructObjectfromClass "/Game/Blueprints/Mechanics/Quests/BP_EnemyKillObjective.BP_EnemyKillObjective_C" (Variables|Default|GetForestSprite6) "Kill Forest Sprite 6" "Kill Forest Sprite 6"))
  (bind _returnvalue_7 (Game|ConstructObjectfromClass "/Game/Blueprints/Mechanics/Quests/BP_EnemyKillObjective.BP_EnemyKillObjective_C" (Variables|Default|GetForestSprite7) "Kill Forest Sprite 7" "Kill Forest Sprite 7"))
  (bind _returnvalue_8 (Game|ConstructObjectfromClass "/Game/Blueprints/Mechanics/Quests/BP_EnemyKillObjective.BP_EnemyKillObjective_C" (Variables|Default|GetForestSprite8) "Kill Forest Sprite 8" "Kill Forest Sprite 8"))
  (bind _returnvalue_9 (Game|ConstructObjectfromClass "/Game/Blueprints/Mechanics/Quests/BP_EnemyKillObjective.BP_EnemyKillObjective_C" (Variables|Default|GetForestSprite9) "Kill Forest Sprite 9" "Kill Forest Sprite 9"))
  (bind _returnvalue_10 (Game|ConstructObjectfromClass "/Game/Blueprints/Mechanics/Quests/BP_EnemyKillObjective.BP_EnemyKillObjective_C" (Variables|Default|GetForestSprite10) "Kill Forest Sprite 10" "Kill Forest Sprite 10"))
  (bind _returnvalue_11 (Game|ConstructObjectfromClass "/Game/Blueprints/Mechanics/Quests/BP_ObjectiveCollection.BP_ObjectiveCollection_C" (Utilities|Array|MakeArray _returnvalue _returnvalue_10 _returnvalue_9 _returnvalue_8 _returnvalue_7 _returnvalue_6 _returnvalue_5 _returnvalue_4 _returnvalue_3 _returnvalue_2) true "Kill Forest Sprites" "KillQuest"))
  (return _returnvalue_11))