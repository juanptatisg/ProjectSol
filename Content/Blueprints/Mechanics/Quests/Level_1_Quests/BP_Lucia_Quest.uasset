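; Level 1 Lucia quest Blueprint that defines its objectives in InitObjectives.
; It constructs item-gathering (Lucia essence), location (Lucia domain) and enemy-kill (Forest Enemy references) objectives.
; Only the kill objective goes into the returned objective collection; the gathering and location objectives are constructed but left out, and share the same objective ID.
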(fn InitObjectives
  (Game|ConstructObjectfromClass "/Game/Blueprints/Mechanics/Quests/BP_ItemGatheringObjective.BP_ItemGatheringObjective_C" 0 (Variables|Default|GetLucia_Essence) 5 "Gather Lucia essence" "Lucia Essence")
  (Game|ConstructObjectfromClass "/Game/Blueprints/Mechanics/Quests/BP_LocationObjective.BP_LocationObjective_C" (Variables|Default|GetLucia_Domain) "Go to Lucia domain" "Lucia Essence")
  (bind _returnvalue (Game|ConstructObjectfromClass "/Game/Blueprints/Mechanics/Quests/BP_EnemyKillObjective.BP_EnemyKillObjective_C" (Utilities|Array|MakeArray (Variables|Default|GetForest_Enemy) (Variables|Default|GetForest_Enemy2) (Variables|Default|GetForest_Enemy3) (Variables|Default|GetForest_Enemy4) (Variables|Default|GetForest_Enemy5)) "Kill Forest Enemy" "KIllEnemy1"))
  (bind _returnvalue_2 (Game|ConstructObjectfromClass "/Game/Blueprints/Mechanics/Quests/BP_ObjectiveCollection.BP_ObjectiveCollection_C" (Utilities|Array|MakeArray _returnvalue)))
  (return _returnvalue_2))