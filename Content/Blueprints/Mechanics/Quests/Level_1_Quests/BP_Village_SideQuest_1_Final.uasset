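; Final village side quest asset for Level 1 that tasks the player with killing ten Forest Sprites.
; InitObjectives builds an enemy kill objective from ten individual sprite references, with a progress bar enabled.
; It wraps that objective in an ordered objective collection and returns it, while the event graph stays empty and construction defers to the parent.
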(event EventBeginPlay)

(event Collision|EventActorBeginOverlap
  (params (OtherActor :type Actor%20Object%20Reference)))

(event EventTick
  (params (DeltaSeconds :type Float%20%28single-precision%29)))

(fn ConstructionScript
  (|CallParentFunction))

(fn InitObjectives
  (bind _returnvalue (Game|ConstructObjectfromClass "/Game/Blueprints/Mechanics/Quests/BP_EnemyKillObjective.BP_EnemyKillObjective_C" (Utilities|Array|MakeArray (Variables|Default|GetForestSprite1) (Variables|Default|GetForestSprite2) (Variables|Default|GetForestSprite3) (Variables|Default|GetForestSprite4) (Variables|Default|GetForestSprite5) (Variables|Default|GetForestSprite6) (Variables|Default|GetForestSprite7) (Variables|Default|GetForestSprite8) (Variables|Default|GetForestSprite9) (Variables|Default|GetForestSprite10)) "Kill 10 Forest Sprites" "Kill Forest Sprites" true))
  (bind _returnvalue_2 (Game|ConstructObjectfromClass "/Game/Blueprints/Mechanics/Quests/BP_ObjectiveCollection.BP_ObjectiveCollection_C" (Utilities|Array|MakeArray _returnvalue) true "Kill Forest Sprites" "KillQuest"))
  (return _returnvalue_2))