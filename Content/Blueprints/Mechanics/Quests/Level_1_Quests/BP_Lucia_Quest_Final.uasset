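; BP_Lucia_Quest_Final is a Level 1 quest Blueprint that defines the objectives for the Lucia quest.
; InitObjectives returns an objective collection whose only sub-objective is killing a set of five forest enemies.
; It also constructs an essence-gathering objective and a Lucia domain location objective, which share an ID but are never added to that collection.
; The event graph holds only disabled stub events.
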(event EventBeginPlay)

(event Collision|EventActorBeginOverlap
  (params (OtherActor :type Actor%20Object%20Reference)))

(event EventTick
  (params (DeltaSeconds :type Float%20%28single-precision%29)))

(fn ConstructionScript
  (|CallParentFunction))

(fn InitObjectives
  (Game|ConstructObjectfromClass "/Game/Blueprints/Mechanics/Quests/BP_ItemGatheringObjective.BP_ItemGatheringObjective_C" 0 (Variables|Default|GetLuciaEssence) 5 "Gather Lucia essence" "Lucia Essence")
  (Game|ConstructObjectfromClass "/Game/Blueprints/Mechanics/Quests/BP_LocationObjective.BP_LocationObjective_C" (Variables|Default|GetLuciaDomain) "Go to Lucia domain" "Lucia Essence")
  (bind _returnvalue (Game|ConstructObjectfromClass "/Game/Blueprints/Mechanics/Quests/BP_EnemyKillObjective.BP_EnemyKillObjective_C" (Utilities|Array|MakeArray (Variables|Default|GetForestEnemy) (Variables|Default|GetForestEnemy2) (Variables|Default|GetForestEnemy3) (Variables|Default|GetForestEnemy4) (Variables|Default|GetForestEnemy5)) "Kill Forest Enemy" "KIllEnemy1"))
  (bind _returnvalue_2 (Game|ConstructObjectfromClass "/Game/Blueprints/Mechanics/Quests/BP_ObjectiveCollection.BP_ObjectiveCollection_C" (Utilities|Array|MakeArray _returnvalue)))
  (return _returnvalue_2))