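; BP_TestQuest2 is a test quest that has the player kill two enemies and then gather an item.
; Its InitObjectives function constructs the objective tree and returns the root: an ordered collection holding an ordered kill collection, followed by an item gathering objective.
; The gathering objective reads the player's inventory component for a configurable item and amount, and shows a progress bar.
; The event graph and construction script add no logic.
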(event EventBeginPlay
  (|CallParentFunction) ; This node is disabled and will not be called.\nDrag off pins to build functionality.
)

(event Collision|EventActorBeginOverlap
  (params (OtherActor :type Actor%20Object%20Reference))
  (|CallParentFunction OtherActor) ; This node is disabled and will not be called.\nDrag off pins to build functionality.
)

(event EventTick
  (params (DeltaSeconds :type Float%20%28single-precision%29))
  (|CallParentFunction DeltaSeconds) ; This node is disabled and will not be called.\nDrag off pins to build functionality.
)

(fn ConstructionScript
  (|CallParentFunction))

(fn InitObjectives
  (bind _returnvalue (Game|ConstructObjectfromClass "/Game/Blueprints/Mechanics/Quests/BP_EnemyKillObjective.BP_EnemyKillObjective_C" (Utilities|Array|MakeArray (Variables|Default|GetEnemy1)) "Kill Enemy 1" "EnemyKill1"))
  (bind _returnvalue_2 (Game|ConstructObjectfromClass "/Game/Blueprints/Mechanics/Quests/BP_EnemyKillObjective.BP_EnemyKillObjective_C" (Utilities|Array|MakeArray (Variables|Default|GetEnemy2)) "Kill Enemy 2" "EnemyKill2"))
  (bind _returnvalue_3 (Game|ConstructObjectfromClass "/Game/Blueprints/Mechanics/Quests/BP_ObjectiveCollection.BP_ObjectiveCollection_C" (Utilities|Array|MakeArray _returnvalue _returnvalue_2) true "KillEnemies" "KillQuest"))
  (bind _asbp_player_base (Utilities|Casting|CastToBP_PlayerBase (Game|GetPlayerCharacter 0)))
  (bind _returnvalue_4 (Game|ConstructObjectfromClass "/Game/Blueprints/Mechanics/Quests/BP_ItemGatheringObjective.BP_ItemGatheringObjective_C" (Variables|/Game/Blueprints/BP_PlayerBase.BP_PlayerBase_C|GetBPC_Inventory _asbp_player_base) (Variables|Default|GetItem%20to%20Look%20For) (Variables|Default|GetAmount%20to%20Get) "GatherItems" "ItemGatheringQuest" true))
  (bind _returnvalue_5 (Game|ConstructObjectfromClass "/Game/Blueprints/Mechanics/Quests/BP_ObjectiveCollection.BP_ObjectiveCollection_C" (Utilities|Array|MakeArray _returnvalue_3 _returnvalue_4) true "SecondTestQuest" "TestQuest2"))
  (return _returnvalue_5))