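; Quest objective Blueprint that tracks how many of a target item get added to the inventory.
; Activation calls the parent, then binds to the InventoryComponent's item-added event.
; The counting function adds one for each matching item, finishing the objective at the required amount or otherwise calling the objective update.
; Completion progress is reported as the ratio of gathered to required amount.
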(fn FActivateObjective
  (|CallParentFunction)
  (EventDispatchers|BindEventtoOnItemAdded (Variables|Default|GetInventoryComponent) (EventDispatchers|CreateEvent :!event FAddItemtoCount)))

(fn FAddItemtoCount
  (params (AddedItem :type BP%20Item%20Object%20Reference))
  (if (== AddedItem (Variables|Default|GetItemToLookFor))
    (bind _output_get (Variables|Default|SetAmountGathered (+ (Variables|Default|GetAmountGathered) 1)))
    (if (>= _output_get (Variables|Default|GetAmountToGet))
      (CallFunction|FFinishObjective)
      (else
        (Default|CallUpdateObjective self)))))

(fn FGetCompletionProgress
  (return (/ (Math|Conversions|ToFloat(Integer) (Variables|Default|GetAmountGathered)) (Math|Conversions|ToFloat(Integer) (Variables|Default|GetAmountToGet)))))