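; BP_JinnEssensePickup is a quest pickup actor that unlocks another stance for the battler when the player touches it.
; A Sphere overlap checks for the first player's pawn, destroys the actor, increments StanceMaxIndex on the referenced battler, then calls the PickedUp dispatcher.
; BeginPlay, Tick and the construction script add no logic of their own.
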(event OnComponentBeginOverlap(Sphere)
  (params (OverlappedComponent :type Primitive%20Component%20Object%20Reference) (OtherActor :type Actor%20Object%20Reference) (OtherComp :type Primitive%20Component%20Object%20Reference) (OtherBodyIndex :type Integer) (bFromSweep :type Boolean) (SweepResult :type Hit%20Result%20Structure%20%28by%20ref%29))
  (bind _battlerref (Variables|Default|GetBattlerRef))
  (if (== OtherActor (Game|Player|GetPlayerPawn 0))
    (Actor|DestroyActor self)
    (bind _result (Math|Integer|IncrementInt (Variables|/Game/Blueprints/BP_PlayerBattler.BP_PlayerBattler_C|GetStanceMaxIndex _battlerref))
      (:%20%20
        (Variables|/Game/Blueprints/BP_PlayerBattler.BP_PlayerBattler_C|SetStanceMaxIndex _battlerref _result)
        (Default|CallPickedUp self)))))

(event EventBeginPlay
  (|CallParentFunction) ; This node is disabled and will not be called.\nDrag off pins to build functionality.
)

(event Collision|EventActorBeginOverlap
  (params (OtherActor :type Actor%20Object%20Reference))
  (|CallParentFunction OtherActor) ; This node is disabled and will not be called.\nDrag off pins to build functionality.
)

(event EventTick
  (params (DeltaSeconds :type Float%20%28single-precision%29)))

(fn ConstructionScript
  (|CallParentFunction))