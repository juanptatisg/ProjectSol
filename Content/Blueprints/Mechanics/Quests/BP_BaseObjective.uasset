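; Base quest objective that tracks active and complete state under an objective ID.
; Activating or finishing sets the matching flag and fires an update or finish event dispatcher, with finishing also printing a debug string.
; Completed IDs can be read out and reapplied by ID lookup, which re-runs the finish path.
; Progress is binary, either zero or one based on completion.
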(fn FActivateObjective
  (Variables|Default|SetIsActive true)
  (Default|CallUpdateObjective self))

(fn FFinishObjective
  (Variables|Default|SetIsComplete true)
  (Default|CallFinishObjective self)
  (Development|PrintString 0 (Utilities|String|Append (Variables|Default|GetObjectiveID) "ObjectiveCompleted")))

(fn FGetCompletedObjectives
  (if (Variables|Default|GetIsComplete)
    (return (Utilities|Array|MakeArray (Variables|Default|GetObjectiveID)))
    (else
      (return 0))))

(fn FSetObjectiveCompletebyID
  (params (CompletedObjectives :type Array%20of%20Strings))
  (if (Utilities|Array|ContainsItem CompletedObjectives (Variables|Default|GetObjectiveID))
    (CallFunction|FFinishObjective)))

(fn FGetCompletionProgress
  (return (Math|Float|SelectFloat 1.0 0.0 (Variables|Default|GetIsComplete))))