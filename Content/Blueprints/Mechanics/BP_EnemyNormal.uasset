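; Sprite-based enemy that chases the player in the overworld, then starts a bullet-pattern battle on contact through the player's Battler.
; Battles spawn bullets in three slots from randomly chosen DataTables, whose rows also set vulnerability.
; Damage scales with defense, vulnerability and combo, builds a decaying stagger meter that interrupts attacks, and can trigger a stat-and-pattern phase switch.
; Death clears bullets and awards level-scaled EXP with looping level-ups before destroying itself.
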(event OnComponentBeginOverlap(EnemyBox)
  (params (OverlappedComponent :type Primitive%20Component%20Object%20Reference) (OtherActor :type Actor%20Object%20Reference) (OtherComp :type Primitive%20Component%20Object%20Reference) (OtherBodyIndex :type Integer) (bFromSweep :type Boolean) (SweepResult :type Hit%20Result%20Structure%20%28by%20ref%29))
  (bind _sprite (Variables|Default|GetSprite))
  (bind _relativescale3d (Variables|/Script/Engine.SceneComponent|GetRelativeScale3D _sprite))
  ;[1 0 0] Initiate Combat
  (if (Math|Boolean|ANDBoolean (not (Variables|Default|GetInCombat)) (Actor|ActorHasTag OtherActor "Player") (not (Components|ComponentHasTag OtherComp "CamBox")))
    (Variables|Default|SetInCombat true)
    (bind _asbp_player_base (Utilities|Casting|CastToBP_PlayerBase OtherActor))
    (Variables|Default|SetPlayerReference _asbp_player_base)
    (Variables|/Game/Blueprints/BP_PlayerBase.BP_PlayerBase_C|SetInCombat _asbp_player_base true)
    (Input|DisableInput (Variables|Default|GetPlayerReference) (Game|GetPlayerController 0))
    (Variables|/Game/Blueprints/BP_PlayerBase.BP_PlayerBase_C|SetMovementState (Variables|Default|GetPlayerReference) "NewEnumerator1")
    (Pawn|Components|CharacterMovement|SetMovementMode (Variables|/Script/Engine.Character|GetCharacterMovement (Variables|Default|GetPlayerReference)) "MOVE_None" 0)
    (Pawn|Components|CharacterMovement|DisableMovement (Variables|Character|GetCharacterMovement))
    (Transformation|SetRelativeScale3D _sprite (Math|Vector|MakeVector (* (Math|Float|Absolute(Float) (.x _relativescale3d)) -1.0) (.y _relativescale3d) (.z _relativescale3d)))
    (Audio|Components|Audio|Stop (Variables|/Script/Paper2D.PaperCharacter|GetSprite (Variables|Default|GetPlayerReference)))
    (Audio|Components|Audio|Stop (Variables|Default|GetSprite))
    (bind _output_get (Variables|Default|SetBattlerRef (Variables|/Game/Blueprints/BP_PlayerBase.BP_PlayerBase_C|GetBattler (Variables|Default|GetPlayerReference))))
    (Variables|/Game/Blueprints/BP_PlayerBattler.BP_PlayerBattler_C|SetCurrentEnemy _output_get self)
    (Default|CreateBattleUI _output_get)
    ;[1 1 1] Setting Bullet Spawners
    (Utilities|FlowControl|Delay 0.2)
    (Variables|Default|SetMiddleSpawn (Variables|/Game/Blueprints/BP_PlayerBattler.BP_PlayerBattler_C|GetMiddleEnemy (Variables|Default|GetBattlerRef)))
    (Variables|Default|SetLeftSpawn (Variables|/Game/Blueprints/BP_PlayerBattler.BP_PlayerBattler_C|GetLeftEnemy (Variables|Default|GetBattlerRef)))
    (Variables|Default|SetRightSpawn (Variables|/Game/Blueprints/BP_PlayerBattler.BP_PlayerBattler_C|GetRightEnemy (Variables|Default|GetBattlerRef)))
    (CallFunction|StartBattle)))

(event OnComponentBeginOverlap(FollowBox)
  (params (OverlappedComponent :type Primitive%20Component%20Object%20Reference) (OtherActor :type Actor%20Object%20Reference) (OtherComp :type Primitive%20Component%20Object%20Reference) (OtherBodyIndex :type Integer) (bFromSweep :type Boolean) (SweepResult :type Hit%20Result%20Structure%20%28by%20ref%29))
  ;[1 0 0.8439] Follow Player
  (if (Actor|ActorHasTag OtherActor "Player")
    (Pawn|Components|CharacterMovement|SetMovementMode (Variables|Character|GetCharacterMovement) "MOVE_Walking" 0)
    (Variables|Default|SetChasing true)
    (bind _asbp_player_base (Utilities|Casting|CastToBP_PlayerBase OtherActor))
    (Variables|Default|SetPlayerReference _asbp_player_base)
    (bind _returnvalue (Utilities|Time|SetTimerbyEvent (delegate Custom|LookForPlayer) 0.01 true true))
    (CallFunction|LookforPlayer)
    (CallFunction|AIFollowPlayer)))

(event OnComponentEndOverlap(FollowBox)
  (params (OverlappedComponent :type Primitive%20Component%20Object%20Reference) (OtherActor :type Actor%20Object%20Reference) (OtherComp :type Primitive%20Component%20Object%20Reference) (OtherBodyIndex :type Integer))
  ;[1 0 0.8439] Follow Player
  (if (Actor|ActorHasTag OtherActor "Player")
    (Variables|Default|SetChasing false)
    (Utilities|Time|PauseTimerbyHandle (stale OnComponentBeginOverlap(FollowBox) _returnvalue))
    (Utilities|Time|ClearandInvalidateTimerbyHandle (stale OnComponentBeginOverlap(FollowBox) _returnvalue))
    (Pawn|Components|CharacterMovement|DisableMovement (Variables|Character|GetCharacterMovement))
    ;[1 0.399 0.6607] Return to Spawn Location
    (if (not (Variables|Default|GetInCombat))
      (Utilities|FlowControl|RetriggerableDelay 3.0)
      (if (not (Variables|Default|GetChasing))
        (Transformation|SetActorLocation self (Variables|Default|GetSpawnPOS) false true)))))

(event Custom|StartBattle
  (bind _battlerref (Variables|Default|GetBattlerRef))
  (bind _staggervalue (Variables|Default|GetStaggerValue))
  (bind _combatui (Variables|/Game/Blueprints/BP_PlayerBattler.BP_PlayerBattler_C|GetCombatUI _battlerref))
  (Rendering|SetVisibility (Variables|Default|GetTextRender) false true)
  (Rendering|SetVisibility (Variables|Default|GetThoughtBubble) false false)
  (Audio|Components|Audio|Play (Variables|Default|GetSprite))
  (Variables|Default|SetIsDead false)
  (Utilities|FlowControl|Delay 2.0)
  (Input|EnableInput (Variables|/Game/Blueprints/BP_PlayerBase.BP_PlayerBase_C|GetBattler (Variables|Default|GetPlayerReference)) (Game|GetPlayerController 0))
  (Collision|SetCollisionResponsetoAllChannels (Variables|Default|GetEnemyBox) "ECR_Ignore")
  (Utilities|Time|SetTimerbyFunctionName 0 "LowerStagger" 0.2 true)
  (bind _selectedattack (CallFunction|ChooseAttackPattern :!label _label))
  (Utilities|FlowControl|DelayUntilNextTick)
  (bind _returnvalue (Utilities|GetDataTableRow _selectedattack (Utilities|String|StringToName (Utilities|String|ToString(Integer) (Variables|Default|GetDataCounter))) :!label _label_2)
    (:then
      (if (or (Variables|Default|GetIsDead) (Utilities|Enum|Equal(Enum) (Variables|Default|GetVulnerablility) "NewEnumerator7"))
        (Utilities|FlowControl|Sequence
          (:then_0
            (Utilities|FlowControl|Sequence
              (:then_0
                (Components|Timeline|SetPlayRate (Variables|Default|GetDepleteStagger) (/ 1.0 (Variables|Default|GetStaggerDuration)))
                (bind _staggerpercent (Timeline|DepleteStagger PlayFromStart)
                  (:Update
                    (Variables|Default|SetCurrentStagger (Math|Float|Round (* _staggervalue _staggerpercent)))
                    (Default|UpdateStagger (Variables|/Game/Blueprints/BP_PlayerBattler.BP_PlayerBattler_C|GetCombatUI (Variables|Default|GetBattlerRef)) (* _staggervalue _staggerpercent) (Math|Conversions|ToFloat(Integer) _staggervalue)))))
              (:then_1
                (bind _opacity (Timeline|StaggerAnim PlayFromStart)
                  (:Update
                    (Default|FlashingStagger _combatui _opacity))))))
          (:then_1
            (Utilities|FlowControl|Delay (Variables|Default|GetStaggerDuration))
            (Utilities|FlowControl|Sequence
              (:then_0
                (Timeline|StaggerAnim Stop))
              (:then_1
                (Variables|Default|SetVulnerablility "NewEnumerator0")
                (Variables|Default|SetCurrentStagger 0)
                (Default|UpdateStagger _combatui 0.0 (Math|Conversions|ToFloat(Integer) (Variables|Default|GetStaggerValue)))
                (Variables|/Script/UMG.Image|SetColorAndOpacity (Variables|/Game/Blueprints/UI/Combat/WBP_CombatUI.WBP_CombatUI_C|GetEnemyStagger _combatui) "(R=1.000000,G=1.000000,B=1.000000,A=1.000000)")
                (Utilities|FlowControl|DelayUntilNextTick)
                (Variables|Default|SetDataCounter 1 :!label _label_3)
                (goto _label)))))
        (else
          (CallFunction|ChangeVulnerability (.Vulnerability (Utilities|Struct|BreakST_BulletData _returnvalue)))
          ;[1 0 0] Spawn Bullet according to its type and slot
          (switch Utilities|FlowControl|Switch|SwitchonENM_BulletSlot (.Slot (Utilities|Struct|BreakST_BulletData _returnvalue))
            (:NewEnumerator0
              (CallFunction|SpawnBullet (.BulletType (Utilities|Struct|BreakST_BulletData _returnvalue)) (.Speed (Utilities|Struct|BreakST_BulletData _returnvalue)) (Variables|Default|GetLeftSpawn)))
            (:NewEnumerator1
              (CallFunction|SpawnBullet (.BulletType (Utilities|Struct|BreakST_BulletData _returnvalue)) (.Speed (Utilities|Struct|BreakST_BulletData _returnvalue)) (Variables|Default|GetMiddleSpawn)))
            (:NewEnumerator2
              (CallFunction|SpawnBullet (.BulletType (Utilities|Struct|BreakST_BulletData _returnvalue)) (.Speed (Utilities|Struct|BreakST_BulletData _returnvalue)) (Variables|Default|GetRightSpawn))))
          (Utilities|FlowControl|Delay (.Delay (Utilities|Struct|BreakST_BulletData _returnvalue)))
          (Math|Integer|IncrementInt (Variables|Default|GetDataCounter)
            (:%20%20
              (goto _label_2))))))
    (:RowNotFound
      (goto _label_3))))

(event Custom|ChangeBarEnemy
  (bind _battlerref (Variables|Default|GetBattlerRef))
  (bind _combatui (Variables|/Game/Blueprints/BP_PlayerBattler.BP_PlayerBattler_C|GetCombatUI _battlerref))
  ;[1 1 1] Bar Gradual alteration
  (bind _loweralpha (Timeline|TimelineEnemy PlayFromStart)
    (:Update
      (Default|ChangeHealthEnemy _combatui _loweralpha)
      (Default|ChangeStagger _combatui _loweralpha))))

(event Custom|LowerStagger
  ;[1 1 1] Bar Gradual alteration
  (if (not (Utilities|Enum|Equal(Enum) (Variables|Default|GetVulnerablility) "NewEnumerator7"))
    (Variables|Default|SetOldStagger (Variables|Default|GetCurrentStagger))
    (bind _output_get (Variables|Default|SetCurrentStagger (- (Variables|Default|GetCurrentStagger) 1)))
    (if (< _output_get 0)
      (Variables|Default|SetCurrentStagger 0))
    (CallFunction|ChangeBarStagger)))

(event Custom|ChangeBarStagger
  ;[1 1 1] Bar Gradual alteration
  (bind _loweralpha (Timeline|Timeline PlayFromStart)
    (:Update
      (Default|ChangeStagger (Variables|/Game/Blueprints/BP_PlayerBattler.BP_PlayerBattler_C|GetCombatUI (Variables|Default|GetBattlerRef)) _loweralpha))))

(event Custom|FinishCombat
  (bind _battlerref (Variables|Default|GetBattlerRef))
  ;[0.7698 0 0] COMBAT END
  ;[1 1 1] Death Animation/Frame
  (Sprite|SetFlipbook (Variables|Default|GetSprite) "/Game/Assets/Scum/Flipbooks/FB_Fire.FB_Fire")
  (Input|DisableInput _battlerref (Game|GetPlayerController 0))
  (Widget|RemovefromParent (Variables|/Game/Blueprints/BP_PlayerBattler.BP_PlayerBattler_C|GetCombatUI _battlerref))
  (bind _outactors (Actor|GetAllActorsOfClass "/Game/Blueprints/Mechanics/BulletLogic/BP_BulletBase.BP_BulletBase_C"))
  (for _array_element _outactors
    (Actor|DestroyActor _array_element))
  (Utilities|FlowControl|Delay 2.0)
  (bind _returnvalue (UserInterface|CreateWidget "/Game/Blueprints/UI/Combat/WBP_EndOfCombat.WBP_EndOfCombat_C" (Game|GetPlayerController 0)))
  (UserInterface|Viewport|AddtoViewport _returnvalue 0)
  (Variables|/Game/Blueprints/UI/Combat/WBP_EndOfCombat.WBP_EndOfCombat_C|SetPlayerRef _returnvalue (Variables|Default|GetBattlerRef))
  (Input|SetInputModeGameandUI (Game|GetPlayerController 0) _returnvalue "DoNotLock" true false)
  (Utilities|FlowControl|Sequence
    (:then_0
      (bind _alpha (Timeline|FadeInWidget PlayFromStart)
        (:Update
          (Appearance|SetColorandOpacity _returnvalue (Utilities|Struct|MakeLinearColor 1.0 1.0 1.0 _alpha) :!class /Script/UMG.UserWidget))))
    (:then_1
      (Utilities|FlowControl|Delay 0.5)
      ;[0.07989 0 1] EXP Raise and Bar
      (bind (_pastexp _newexp _leftover) (CallFunction|GivePlayerEXP (Math|Float|SelectFloat (Variables|Default|GetLeftoverStorage) (Variables|Default|GetEXPYield) (Variables|Default|GetLoopingLevelup)) :!label _label))
      (Variables|Default|SetLeftoverStorage _leftover)
      (Components|Timeline|SetPlayRate (Variables|Default|GetIncreaseEXP) (/ 4e+02 (- _newexp _pastexp)))
      (bind _alpha_2 (Timeline|IncreaseEXP PlayFromStart)
        (:Update
          (Default|ChangeBarEXP _returnvalue _pastexp _newexp _alpha_2))
        (:Finished
          (if (>= (Variables|Default|GetLeftoverStorage) 0.0)
            (Default|LevelUp (Variables|Default|GetBattlerRef))
            (Variables|Default|SetLoopingLevelup true)
            (goto _label)
            (else
              (Variables|/Game/Blueprints/UI/Combat/WBP_EndOfCombat.WBP_EndOfCombat_C|SetCompleted _returnvalue true)
              (Utilities|FlowControl|DelayUntilNextTick)
              (Actor|DestroyActor))))))))

(event Custom|AIFollowPlayer
  ;[1 0 0.8439] Follow Player
  (Development|PrintString "following player")
  (AI|AIMoveTo self (Variables|Default|GetPlayerPOS) (Variables|Default|GetPlayerReference) 5.0 false
    (:OnSuccess
      (Development|PrintString "following!!"))
    (:OnFail
      (Development|PrintString "cant move"))))

(event Custom|LookForPlayer
  (bind _playerreference (Variables|Default|GetPlayerReference))
  ;[1 0 0.8439] Follow Player
  (if (Utilities|IsValid _playerreference)
    (if (Variables|/Game/Blueprints/BP_PlayerBase.BP_PlayerBase_C|GetInCombat _playerreference)
      (Utilities|Time|PauseTimerbyHandle (stale OnComponentBeginOverlap(FollowBox) _returnvalue))
      (Utilities|Time|ClearandInvalidateTimerbyHandle (stale OnComponentBeginOverlap(FollowBox) _returnvalue))
      (Pawn|Components|CharacterMovement|DisableMovement (Variables|Character|GetCharacterMovement))
      ;[1 0.399 0.6607] Return to Spawn Location
      (if (not (Variables|Default|GetInCombat))
        (Utilities|FlowControl|RetriggerableDelay 3.0)
        (if (not (Variables|Default|GetChasing))
          (Transformation|SetActorLocation self (Variables|Default|GetSpawnPOS) false true)))
      (else
        (Variables|Default|SetPlayerPOS (Transformation|GetWorldLocation (Variables|/Script/Engine.Character|GetCapsuleComponent _playerreference)))
        (CallFunction|UpdateRotation)))))

(event Custom|Vibrate
  (bind _battleposition (Variables|Default|GetBattlePosition))
  ;[1 1 1] Vibrate
  (bind _vibrationoffset (Timeline|DamageVibrate PlayFromStart)
    (:Update
      (Transformation|SetActorLocation (Math|Vector|MakeVector (+ (.x _battleposition) _vibrationoffset) (.y _battleposition) (.z _battleposition)) false true))
    (:Finished
      (Transformation|SetActorLocation (Variables|Default|GetBattlePosition) false true))))

(event EventBeginPlay
  (bind _stats (Variables|Default|GetStats))
  (bind _level (Utilities|Struct|BreakST_Stats _stats))
  (bind _returnvalue (Utilities|String|ToString(Integer) _level))
  (bind _returnvalue_2 (Utilities|String|Append "Lv." _returnvalue))
  (bind _returnvalue_3 (Utilities|Text|ToText(String) _returnvalue_2))
  (Variables|Default|SetCurrentHealth (.maxhp (Variables|Default|GetStats)))
  (Variables|Default|SetCurrentStagger 0)
  (Variables|Default|SetSpawnPOS (Transformation|GetActorLocation))
  (Rendering|Components|TextRender|SetText (Variables|Default|GetTextRender) _returnvalue_3)
  (Rendering|Components|TextRender|SetText (Variables|Default|GetTextOutline) _returnvalue_3))

(fn ConstructionScript)

(fn SpawnBullet
  (params (BulletType :type Actor%20Class%20Reference) (Speed :type Float%20%28double-precision%29) (Slot :type Paper%20Sprite%20Component%20Object%20Reference))
  (bind _returnvalue (Game|SpawnActorfromClass BulletType (Transformation|GetWorldTransform Slot) "AlwaysSpawn" "MultiplyWithRoot" 0 0))
  (bind _asbp_bullet_base (Utilities|Casting|CastToBP_BulletBase _returnvalue))
  (Variables|/Game/Blueprints/Mechanics/BulletLogic/BP_BulletBase.BP_BulletBase_C|SetSpeed _asbp_bullet_base Speed))

(fn ChooseAttackPattern
  (bind _phaseindex (Variables|Default|GetPhaseIndex))
  (bind _attackarray (Variables|Default|GetAttackArray))
  (bind _attackarrayalt (Variables|Default|GetAttackArrayAlt))
  (bind _returnvalue (Utilities|Select :Index _phaseindex :Option%200 _attackarray :Option%201 _attackarrayalt))
  (return (Utilities|Array|Get(acopy) _returnvalue (Math|Random|RandomIntegerinRange 0 (- (Utilities|Array|Length _returnvalue) 1)))))

(fn TakeDamageEnemy
  (params (DamageTaken :type Float%20%28double-precision%29) (StaggerDamage :type Integer) (StaggerMultiplier :type Float%20%28double-precision%29))
  (bind _battlerref (Variables|Default|GetBattlerRef))
  (bind _capsule (Variables|Default|GetCapsule))
  (bind _stats (Variables|Default|GetStats))
  (bind _battlerref_2 (Variables|Default|GetBattlerRef))
  (bind _returnvalue (Transformation|GetWorldLocation _capsule))
  (bind _combocounter (Variables|/Game/Blueprints/BP_PlayerBattler.BP_PlayerBattler_C|GetComboCounter _battlerref_2))
  (bind (_x _y _z) (Math|Vector|BreakVector _returnvalue))
  (bind _returnvalue_2 (Math|Conversions|ToFloat(Integer) _combocounter))
  (bind _returnvalue_3 (/ _combocounter 300))
  (bind _returnvalue_4 (/ _returnvalue_2 2.0))
  (bind _returnvalue_5 (+ _returnvalue_3 1.0))
  (bind _output_get (Variables|Default|SetOldHealth (Variables|Default|GetCurrentHealth)))
  (Variables|Default|SetOldStagger (Variables|Default|GetCurrentStagger))
  (Development|PrintString (Utilities|String|ToString(Float) DamageTaken))
  (CallFunction|Vibrate)
  (bind _output_get_2 (Variables|Default|SetCurrentHealth (Math|Conversions|ToFloat(Integer) (Math|Float|Round (Utilities|Operators|Subtract (Variables|Default|GetCurrentHealth) (Math|Float|SelectFloat (* (/ (- DamageTaken (/ (.defense _stats) 4.0)) (/ (.defense _stats) 25.0)) (Utilities|Select :Index (Variables|Default|GetVulnerablility) :NewEnumerator0 1.0 :NewEnumerator5 (Variables|Default|GetVulnerableMod) :NewEnumerator6 0.7 :NewEnumerator7 (Variables|Default|GetStaggerMod))) 1.0 (> (* (/ (- DamageTaken (/ (.defense _stats) 4.0)) (/ (.defense _stats) 25.0)) (Utilities|Select :Index (Variables|Default|GetVulnerablility) :NewEnumerator0 1.0 :NewEnumerator5 (Variables|Default|GetVulnerableMod) :NewEnumerator6 0.7 :NewEnumerator7 (Variables|Default|GetStaggerMod))) 0.0)) (Math|Float|SelectFloat (Math|Float|SelectFloat 1.5e+02 _returnvalue_4 (> _returnvalue_4 1.5e+02)) 0.0 (Utilities|Enum|Equal(Enum) (Variables|/Game/Blueprints/BP_PlayerBattler.BP_PlayerBattler_C|GetAuraEnum (Variables|Default|GetBattlerRef)) "NewEnumerator1")))))))
  (if (<= _output_get_2 0.0)
    (Variables|Default|SetCurrentHealth 0.0)
    (Variables|Default|SetCurrentStagger 0)
    (Utilities|FlowControl|Sequence
      (:then_0
        (Utilities|FlowControl|Sequence :!label _label
          (:then_0
            (if (Utilities|Enum|Equal(Enum) (Variables|Default|GetVulnerablility) "NewEnumerator7")
              (Utilities|FlowControl|Sequence :!label _label_2
                (:then_0
                  (if (<= (/ (Variables|Default|GetCurrentHealth) (.MaxHP (Utilities|Struct|BreakST_Stats (Variables|Default|GetStats)))) (Variables|Default|GetPhaseSwitchPercent))
                    (CallFunction|SwitchPhase)))
                (:then_1
                  (bind _returnvalue_6 (Game|SpawnActorfromClass "/Game/Blueprints/UI/Combat/BP_DamageNumbers.BP_DamageNumbers_C" (Math|Transform|MakeTransform (Math|Vector|MakeVector (+ _x -75.0) (+ _y 1e+02) (- _z -2e+02)) "0.000000,90.000000,0.000000" "0.700000,0.700000,0.700000") "Undefined" "MultiplyWithRoot" 0 0))
                  (Rendering|Components|TextRender|SetText (Variables|/Game/Blueprints/UI/Combat/BP_DamageNumbers.BP_DamageNumbers_C|GetTextRender _returnvalue_6) (Utilities|Text|ToText(Float) (- _output_get _output_get_2) "HalfToEven"))
                  (if (> StaggerMultiplier 1.0)
                    (Rendering|Components|TextRender|SetTextRenderColor (Variables|/Game/Blueprints/UI/Combat/BP_DamageNumbers.BP_DamageNumbers_C|GetTextRender _returnvalue_6) (Math|Conversions|ToColor(LinearColor) "(R=1.000000,G=0.000000,B=0.000000,A=1.000000)")))))))
          (:then_1
            (goto _label_2))))
      (:then_1
        (Variables|Default|SetIsDead true)
        (CallFunction|FinishCombat)))
    (else
      (bind _output_get_3 (Variables|Default|SetCurrentStagger (+ (Variables|Default|GetCurrentStagger) (* (* (* StaggerDamage StaggerMultiplier) (Math|Float|SelectFloat 4.0 _returnvalue_5 (> _returnvalue_5 4.0))) (Utilities|Select :Index (Variables|Default|GetVulnerablility) :NewEnumerator0 1.0 :NewEnumerator5 1.5 :NewEnumerator6 0.0 :NewEnumerator7 1.0)))))
      (if (>= _output_get_3 (Variables|Default|GetStaggerValue))
        ;[1 1 1] Max Energy on Stagger
        (Variables|Default|SetCurrentStagger (Variables|Default|GetStaggerValue))
        (if (Utilities|Enum|NotEqual(Enum) (Variables|Default|GetVulnerablility) "NewEnumerator7")
          (Variables|Default|SetVulnerablility "NewEnumerator7")
          (Variables|/Game/Blueprints/BP_PlayerBattler.BP_PlayerBattler_C|SetCurrentEnergy _battlerref 1e+02)
          (Default|ChangeBarEnergy _battlerref)
          (Default|StaggerEffect _battlerref)
          (goto _label)
          (else
            (goto _label)))
        (else
          (goto _label))))))

(fn ChangeVulnerability
  (params (Vulnerability :type ENM_Vulnerability%20Enum :default "NewEnumerator0"))
  (bind _thoughtbubble (Variables|Default|GetThoughtBubble))
  (bind _output_get (Variables|Default|SetVulnerablility Vulnerability))
  (switch Utilities|FlowControl|Switch|SwitchonENM_Vulnerability _output_get
    (:NewEnumerator0
      (Sprite|SetSpriteColor _thoughtbubble "(R=1.000000,G=1.000000,B=1.000000,A=1.000000)"))
    (:NewEnumerator5
      (Sprite|SetSpriteColor _thoughtbubble "(R=1.000000,G=0.985022,B=0.000000,A=1.000000)"))
    (:NewEnumerator6
      (Sprite|SetSpriteColor _thoughtbubble "(R=0.000000,G=0.034567,B=1.000000,A=1.000000)"))
    (:NewEnumerator7
      (Sprite|SetSpriteColor _thoughtbubble "(R=0.931250,G=0.067904,B=0.067904,A=1.000000)"))))

(fn GainHealthEnemy
  (params (HealPercent :type Float%20%28double-precision%29))
  (bind _returnvalue (Math|Random|RandomFloatinRange 0.9 1.0))
  (bind _returnvalue_2 (* HealPercent 1e+02))
  (bind _stats (Variables|Default|GetStats))
  (bind _capsule (Variables|Default|GetCapsule))
  (bind _stats_2 (Variables|Default|GetStats))
  (bind _maxhp (Utilities|Struct|BreakST_Stats _stats))
  (bind (_level _maxhp_2 _energy _attack _defense _healing) (Utilities|Struct|BreakST_Stats _stats_2))
  (bind _returnvalue_3 (Transformation|GetWorldLocation _capsule))
  (bind (_x _y _z) (Math|Vector|BreakVector _returnvalue_3))
  (bind _returnvalue_4 (* HealPercent _maxhp_2))
  (bind _returnvalue_5 (* _healing _returnvalue_2))
  (bind _returnvalue_6 (+ _returnvalue_4 _returnvalue_5))
  (bind _returnvalue_7 (* _returnvalue_6 _returnvalue))
  (bind _returnvalue_8 (Math|Float|Round _returnvalue_7))
  (bind _returnvalue_9 (Math|Conversions|ToFloat(Integer) _returnvalue_8))
  (Variables|Default|SetOldHealth (Variables|Default|GetCurrentHealth))
  (bind _output_get (Variables|Default|SetCurrentHealth (+ _returnvalue_9 (Variables|Default|GetCurrentHealth))))
  (if (> _output_get _maxhp)
    (Variables|Default|SetCurrentHealth _maxhp))
  (bind _returnvalue_10 (Game|SpawnActorfromClass "/Game/Blueprints/UI/Combat/BP_DamageNumbers.BP_DamageNumbers_C" (Math|Transform|MakeTransform (Math|Vector|MakeVector (+ _x -75.0) (+ _y 1e+02) (- _z -2e+02)) "0.000000,90.000000,0.000000" "0.700000,0.700000,0.700000") "Undefined" "MultiplyWithRoot" 0 0))
  (Rendering|Components|TextRender|SetText (Variables|/Game/Blueprints/UI/Combat/BP_DamageNumbers.BP_DamageNumbers_C|GetTextRender _returnvalue_10) (Utilities|Text|ToText(Float) _returnvalue_9 "HalfToEven"))
  (Rendering|Components|TextRender|SetTextRenderColor (Variables|/Game/Blueprints/UI/Combat/BP_DamageNumbers.BP_DamageNumbers_C|GetTextRender _returnvalue_10) (Math|Conversions|ToColor(LinearColor) "(R=0.000000,G=1.000000,B=0.100000,A=1.000000)")))

(fn GivePlayerEXP
  (params (EXPAmount :type Float%20%28double-precision%29))
  (bind _battlerref (Variables|Default|GetBattlerRef))
  (bind _battlerref_2 (Variables|Default|GetBattlerRef))
  (bind _battlerref_3 (Variables|Default|GetBattlerRef))
  (bind _battlerref_4 (Variables|Default|GetBattlerRef))
  (bind _stats (Variables|Default|GetStats))
  (bind _battlerref_5 (Variables|Default|GetBattlerRef))
  (bind _level (Utilities|Struct|BreakST_Stats _stats))
  (bind _statsbase (Variables|/Game/Blueprints/BP_PlayerBattler.BP_PlayerBattler_C|GetStatsBase _battlerref_5))
  (bind _level_2 (Utilities|Struct|BreakST_Stats _statsbase))
  (bind _returnvalue (- _level_2 _level))
  (bind _returnvalue_2 (Math|Integer|Absolute(Integer) _returnvalue))
  (bind _returnvalue_3 (Math|Conversions|ToFloat(Integer) _returnvalue_2))
  (bind _returnvalue_4 (Math|Float|Power 1.2 _returnvalue_3))
  (Development|PrintString (Utilities|String|ToString(Float) EXPAmount))
  (if (>= (Variables|/Game/Blueprints/BP_PlayerBattler.BP_PlayerBattler_C|GetExperience _battlerref_3) 1e+03)
    (Variables|/Game/Blueprints/BP_PlayerBattler.BP_PlayerBattler_C|SetExperience _battlerref_3 0.0))
  (LocalVariables|SetOldEXP (Variables|/Game/Blueprints/BP_PlayerBattler.BP_PlayerBattler_C|GetExperience (Variables|Default|GetBattlerRef)))
  (if (< _returnvalue 0)
    (if (Variables|Default|GetLoopingLevelup)
      ;[1 1 1] Discard Level Diff Multiplier
      (Variables|/Game/Blueprints/BP_PlayerBattler.BP_PlayerBattler_C|SetExperience _battlerref (Math|Conversions|ToFloat(Integer) (Math|Float|Round (+ EXPAmount (Variables|/Game/Blueprints/BP_PlayerBattler.BP_PlayerBattler_C|GetExperience _battlerref)))))
      (else
        (Development|PrintString (Utilities|String|ToString(Float) (Math|Conversions|ToFloat(Integer) (Math|Float|Round (+ (* EXPAmount (Math|Float|SelectFloat 4.0 _returnvalue_4 (> _returnvalue_4 4.0))) (Variables|/Game/Blueprints/BP_PlayerBattler.BP_PlayerBattler_C|GetExperience _battlerref_4))))))
        ;[0 1 1] Enemy Higher Level
        (Variables|/Game/Blueprints/BP_PlayerBattler.BP_PlayerBattler_C|SetExperience _battlerref_4 (Math|Conversions|ToFloat(Integer) (Math|Float|Round (+ (* EXPAmount (Math|Float|SelectFloat 4.0 _returnvalue_4 (> _returnvalue_4 4.0))) (Variables|/Game/Blueprints/BP_PlayerBattler.BP_PlayerBattler_C|GetExperience _battlerref_4)))))))
    (else
      ;[1 0 1] Enemy Lower Level
      (Variables|/Game/Blueprints/BP_PlayerBattler.BP_PlayerBattler_C|SetExperience _battlerref_2 (Math|Conversions|ToFloat(Integer) (Math|Float|Round (+ (/ EXPAmount (Math|Float|Power 1.5 (Math|Conversions|ToFloat(Integer) (Math|Integer|Absolute(Integer) (- (.Level (Utilities|Struct|BreakST_Stats (Variables|/Game/Blueprints/BP_PlayerBattler.BP_PlayerBattler_C|GetStatsBase (Variables|Default|GetBattlerRef)))) (.Level (Utilities|Struct|BreakST_Stats (Variables|Default|GetStats)))))))) (Variables|/Game/Blueprints/BP_PlayerBattler.BP_PlayerBattler_C|GetExperience _battlerref_2)))))))
  (if (> (Variables|/Game/Blueprints/BP_PlayerBattler.BP_PlayerBattler_C|GetExperience (Variables|Default|GetBattlerRef)) 999.0)
    (return (LocalVariables|GetOldEXP) 1e+03 (- (Variables|/Game/Blueprints/BP_PlayerBattler.BP_PlayerBattler_C|GetExperience (Variables|Default|GetBattlerRef)) 1e+03))
    (else
      (return (LocalVariables|GetOldEXP) (Variables|/Game/Blueprints/BP_PlayerBattler.BP_PlayerBattler_C|GetExperience (Variables|Default|GetBattlerRef)) -1.0))))

(fn UpdateRotation
  (bind _sprite (Variables|Default|GetSprite))
  (bind _sprite_2 (Variables|Default|GetSprite))
  (bind _relativescale3d (Variables|/Script/Engine.SceneComponent|GetRelativeScale3D _sprite))
  (bind _relativescale3d_2 (Variables|/Script/Engine.SceneComponent|GetRelativeScale3D _sprite_2))
  (Math|Float|CompareFloat (.x (Transformation|GetVelocity)) 0.0
    (:>
      (Transformation|SetRelativeScale3D _sprite_2 (Math|Vector|MakeVector (* (Math|Float|SelectFloat -1.0 1.0 (< (.x _relativescale3d_2) 0.0)) (.x _relativescale3d_2)) (.y _relativescale3d_2) (.z _relativescale3d_2))))
    (:<
      (Transformation|SetRelativeScale3D _sprite (Math|Vector|MakeVector (* (Math|Float|SelectFloat -1.0 1.0 (> (.x _relativescale3d) 0.0)) (.x _relativescale3d)) (.y _relativescale3d) (.z _relativescale3d))))))

(fn SwitchPhase
  (bind _statsalt (Variables|Default|GetStatsAlt))
  (Development|PrintString "PHASE SWITCH")
  (Math|Integer|IncrementInt (Variables|Default|GetPhaseIndex)
    (:%20%20
      (Variables|Default|SetPhaseSwitchPercent -1.0)
      (Variables|Default|SetStats (Utilities|Struct|MakeST_Stats (.level _statsalt) (.maxhp _statsalt) (.energy _statsalt) (.attack _statsalt) (.defense _statsalt) (.healing _statsalt) (.critrate _statsalt) (.energygain _statsalt))))))