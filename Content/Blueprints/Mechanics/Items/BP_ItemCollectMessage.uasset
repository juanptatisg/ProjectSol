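; BP_ItemCollectMessage is a short-lived floating text actor, named as the message for item collection.
; On BeginPlay it waits one tick, then plays a timeline whose OffsetZ value is added to the actor's height on each update, and destroys itself when the timeline finishes.
; Tick grows the TextRender's world scale by a fixed step every frame, so the growth rate depends on frame rate.
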(event EventBeginPlay
  (Utilities|FlowControl|DelayUntilNextTick)
  (bind _offsetz (Timeline|movementTimeline PlayFromStart)
    (:Update
      (Transformation|AddActorWorldOffset (Math|Vector|MakeVector 0.0 0.0 _offsetz)))
    (:Finished
      (Actor|DestroyActor))))

(event EventTick
  (params (DeltaSeconds :type Float%20%28single-precision%29))
  (bind _textrender (Variables|Default|GetTextRender))
  (bind _returnvalue (Transformation|GetWorldScale _textrender))
  (bind (_x _y _z) (Math|Vector|BreakVector _returnvalue))
  (Transformation|SetWorldScale3D _textrender (Math|Vector|MakeVector (+ _x 0.01) (+ _y 0.01) (+ _z 0.01))))

(fn ConstructionScript)