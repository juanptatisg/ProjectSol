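; Inventory component whose AddItem adds items to its owner's inventory, capped at 99 entries.
; Item classes and their display, quantity and modifier data live in parallel arrays matched by index.
; Duplicates only stack quantity for one item type; new classes are appended and trigger an item-added call.
; A new Fate, Hope, Life or Love Remnant also raises the player Battler's maximum stance index.
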(fn AddItem
  (params (NewItem :type BP%20Item%20Object%20Reference%20%28by%20ref%29))
  (bind _inventory (Variables|Default|GetInventory))
  (bind _dataindexes (Variables|Default|GetDataIndexes))
  (bind _returnvalue (Utilities|GetClass NewItem))
  (bind _returnvalue_2 (Utilities|GetClass NewItem))
  (bind _returnvalue_3 (Utilities|Array|FindItem _inventory _returnvalue_2))
  (bind _output (Utilities|Array|Get(acopy) _dataindexes _returnvalue_3))
  (if (< (Utilities|Array|Length (Variables|Default|GetInventory)) 99)
    (if (Utilities|Array|ContainsItem (Variables|Default|GetInventory) (Utilities|GetClass NewItem))
      (if (Utilities|Enum|Equal(Enum) (Variables|/Game/Blueprints/Mechanics/BP_Item.BP_Item_C|GetItemType NewItem) "NewEnumerator0")
        (Utilities|Array|SetArrayElem (Variables|Default|GetDataIndexes) _returnvalue_3 (Utilities|Struct|MakeSTR_ItemData (.name _output) (.description _output) (.icon _output) (.type _output) (+ (.quantity _output) (Variables|/Game/Blueprints/Mechanics/BP_Item.BP_Item_C|GetQuantity NewItem)) (.modifiers _output))))
      (elif (Utilities|IsValid NewItem)
        (bind _returnvalue_4 (Utilities|Array|Add (Variables|Default|GetInventory) (Utilities|GetClass NewItem)))
        (Default|CallOnItemAdded NewItem)
        (Utilities|Array|SetArrayElem (Variables|Default|GetDataIndexes) _returnvalue_4 (Utilities|Struct|MakeSTR_ItemData (Variables|/Game/Blueprints/Mechanics/BP_Item.BP_Item_C|GetItemName NewItem) (Variables|/Game/Blueprints/Mechanics/BP_Item.BP_Item_C|GetItemDescription NewItem) (Variables|/Game/Blueprints/Mechanics/BP_Item.BP_Item_C|GetItemImage NewItem) (Variables|/Game/Blueprints/Mechanics/BP_Item.BP_Item_C|GetItemType NewItem) (Variables|/Game/Blueprints/Mechanics/BP_Item.BP_Item_C|GetQuantity NewItem) (Variables|/Game/Blueprints/Mechanics/BP_Item.BP_Item_C|GetItemModifiers NewItem)) true)
        (bind _asbp_player_base (Utilities|Casting|CastToBP_PlayerBase (Components|GetOwner)))
        (if (Math|Boolean|ORBoolean (== _returnvalue "/Game/Blueprints/Mechanics/Items/KeyItems/BP_FateRemnant.BP_FateRemnant_C") (== _returnvalue "/Game/Blueprints/Mechanics/Items/KeyItems/BP_HopeRemnant.BP_HopeRemnant_C") (== _returnvalue "/Game/Blueprints/Mechanics/Items/KeyItems/BP_LifeRemnant.BP_LifeRemnant_C") (== _returnvalue "/Game/Blueprints/Mechanics/Items/KeyItems/BP_LoveRemnant.BP_LoveRemnant_C"))
          (Math|Integer|IncrementInt (Variables|/Game/Blueprints/BP_PlayerBattler.BP_PlayerBattler_C|GetStanceMaxIndex (Variables|/Game/Blueprints/BP_PlayerBase.BP_PlayerBase_C|GetBattler _asbp_player_base))))
        (else
          (Development|PrintString "NOITEM"))))))