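; BP_BulletVanish is a bullet variant that gradually fades out after it spawns.
; One tick after BeginPlay, it starts a looping timer whose interval shrinks as Speed rises, so faster bullets fade sooner.
; Each Vanish call lowers the BulletSprite alpha by a fixed step, keeping its RGB.
; This graph never clears the timer or destroys the actor, and all other behavior comes from the parent class.
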(event Custom|Vanish
  (bind _bulletsprite (Variables|Default|GetBulletSprite))
  (bind _spritecolor (Variables|/Script/Paper2D.PaperSpriteComponent|GetSpriteColor _bulletsprite))
  (Sprite|SetSpriteColor _bulletsprite (Utilities|Struct|MakeLinearColor (.r _spritecolor) (.g _spritecolor) (.b _spritecolor) (- (.a _spritecolor) 0.025))))

(event EventBeginPlay
  (|CallParentFunction)
  (Utilities|FlowControl|DelayUntilNextTick)
  (Utilities|Time|SetTimerbyEvent (delegate Custom|Vanish) (/ 0.2 (Variables|Default|GetSpeed)) true)
  (CallFunction|Vanish))

(event EventTick
  (params (DeltaSeconds :type Float%20%28single-precision%29))
  (|CallParentFunction DeltaSeconds) ; This node is disabled and will not be called.\nDrag off pins to build functionality.
)

(fn ConstructionScript
  (|CallParentFunction))