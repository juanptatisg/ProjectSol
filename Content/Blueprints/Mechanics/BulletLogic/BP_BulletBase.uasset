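; BP_BulletBase is a bullet actor that moves down world Z each tick and damages the player battler on hit.
; Movement is an unswept sprite offset scaled by Speed but not delta time, and the bullet self-destroys after a Speed-scaled delay.
; On overlap, HitBoxL looks for "Hurtbox"-tagged components, plays a hit sound, passes damage and bullet type to BP_PlayerBattler, then updates its bar and destroys itself across following ticks.
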(event EventBeginPlay
  (Utilities|FlowControl|Delay (* 1e+01 (Variables|Default|GetSpeed)))
  (Actor|DestroyActor))

(event Collision|EventActorBeginOverlap
  (params (OtherActor :type Actor%20Object%20Reference))
  (bind _hitboxl (Variables|Default|GetHitBoxL))
  (Utilities|IsValid _hitboxl
    (:Is%20Valid
      (for _array_element (Class|PrimitiveComponent|GetOverlappingComponents _hitboxl)
        (if (Components|ComponentHasTag _array_element "Hurtbox")
          (Audio|PlaySound2D "/Game/Assets/MEchoes/Audio/SFX/DeathHit.DeathHit" 1.0 1.0 0.0 "/Game/Assets/Audio/SC_BattleEffects.SC_BattleEffects" 0)
          (bind _asbp_player_battler (Utilities|Casting|CastToBP_PlayerBattler OtherActor))
          (Default|TakeDamage _asbp_player_battler (Variables|Default|GetBaseDamage) (Variables|Default|GetType))
          (Utilities|FlowControl|DelayUntilNextTick)
          (Default|ChangeBarDamaged _asbp_player_battler)
          (Utilities|FlowControl|DelayUntilNextTick)
          (Actor|DestroyActor))))))

(event EventTick
  (params (DeltaSeconds :type Float%20%28single-precision%29))
  (Transformation|AddWorldOffset (Variables|Default|GetBulletSprite) (Math|Vector|MakeVector 0.0 0.0 (* (Variables|Default|GetSpeed) -1.0)) false false))

(fn ConstructionScript)