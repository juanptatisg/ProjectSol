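; Bullet variant that teleports sideways up to three times during its flight, jumping between three X positions around its starting point.
; After an initial delay, a looping timer drives WarpAround at an interval inversely proportional to Speed.
; Each warp resets the sprite to its starting X and Y, keeps its current Z, then applies an offset picked from a shuffled index array, which swaps entries with SelectedIndex.
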(event Custom|WarpAround
  (bind _bulletsprite (Variables|Default|GetBulletSprite))
  (bind _indexarray (Variables|Default|GetIndexArray))
  (bind _startingpoint (Variables|Default|GetStartingPoint))
  (bind _indexarray_2 (Variables|Default|GetIndexArray))
  (bind _output (Utilities|Array|Get(acopy) _indexarray_2))
  (if (< (Variables|Default|GetCounter) 3)
    (Utilities|Array|Shuffle (Variables|Default|GetIndexArray))
    (Transformation|SetWorldLocation _bulletsprite (Math|Vector|MakeVector (.x _startingpoint) (.y _startingpoint) (.z (Transformation|GetWorldLocation (Variables|Default|GetBulletSprite)))) false true)
    (Transformation|AddWorldOffset _bulletsprite (Math|Vector|MakeVector (Utilities|Select :Index _output :Option%200 -79.8 :Option%201 0.0 :Option%202 79.8) 0.0 0.0) false true)
    (Math|Integer|IncrementInt (Variables|Default|GetCounter)
      (:%20%20
        (Utilities|Array|RemoveItem _indexarray _output)
        (Utilities|Array|Add _indexarray (Variables|Default|GetSelectedIndex))
        (Variables|Default|SetSelectedIndex _output)))))

(event EventBeginPlay
  (bind _speed (Variables|Default|GetSpeed))
  (bind _returnvalue (/ 1.75 _speed))
  (|CallParentFunction)
  (Utilities|FlowControl|DelayUntilNextTick)
  (Variables|Default|SetStartingPoint (Transformation|GetWorldLocation (Variables|Default|GetBulletSprite)))
  (Variables|Default|SetCounter 0)
  (Utilities|FlowControl|Delay _returnvalue)
  (Utilities|Time|SetTimerbyEvent (delegate Custom|WarpAround) _returnvalue true)
  (CallFunction|WarpAround))

(fn ConstructionScript
  (|CallParentFunction))