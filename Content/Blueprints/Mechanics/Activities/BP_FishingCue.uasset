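; BP_FishingCue is the visual bite cue for the fishing activity, signalling when to react after a random wait.
; While waiting, Tick pulses the white Cue sprite's alpha in and out.
; After the delay it turns blue, plays a high-pitched jump sound and prints NOW, then fades out each frame at a rate divided by Difficulty.
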(event EventBeginPlay
  (Variables|Default|SetWaiting true)
  (Sprite|SetSpriteColor (Variables|Default|GetCue) (Math|Color|MakeColor 1.0 1.0 1.0 0.0))
  (bind _output_get (Variables|Default|SetHitDelay (Math|Random|RandomFloatinRange 3.0 8.0)))
  (Utilities|FlowControl|Delay _output_get)
  (if (Variables|Default|GetWaiting)
    (Variables|Default|SetWaiting false)
    (Sprite|SetSpriteColor (Variables|Default|GetCue) (Math|Color|MakeColor 0.0 0.0 1.0))
    (Development|PrintString "NOW")
    (Audio|PlaySound2D "/Game/Assets/MEchoes/Audio/SFX/JumpEffect.JumpEffect" 1.3 4.0 0.02 0 0)))

(event EventTick
  (params (DeltaSeconds :type Float%20%28single-precision%29))
  (bind _cue (Variables|Default|GetCue))
  (bind _cue_2 (Variables|Default|GetCue))
  (bind _cue_3 (Variables|Default|GetCue))
  (bind _spritecolor (Variables|/Script/Paper2D.PaperSpriteComponent|GetSpriteColor _cue_3))
  (bind _spritecolor_2 (Variables|/Script/Paper2D.PaperSpriteComponent|GetSpriteColor _cue_2))
  (bind _spritecolor_3 (Variables|/Script/Paper2D.PaperSpriteComponent|GetSpriteColor _cue))
  (bind _a (Math|Color|BreakColor _spritecolor))
  (bind (_r _g _b _a_2) (Math|Color|BreakColor _spritecolor_2))
  (bind _a_3 (Math|Color|BreakColor _spritecolor_3))
  (bind _returnvalue (+ _a_3 0.025))
  (bind _returnvalue_2 (- _a 0.025))
  (if (Variables|Default|GetWaiting)
    (if (Variables|Default|GetGrowing)
      (Sprite|SetSpriteColor _cue (Math|Color|MakeColor 1.0 1.0 1.0 _returnvalue))
      (if (>= _returnvalue 1.0)
        (Variables|Default|SetGrowing false))
      (else
        (Sprite|SetSpriteColor _cue_3 (Math|Color|MakeColor 1.0 1.0 1.0 _returnvalue_2))
        (if (<= _returnvalue_2 0.0)
          (Variables|Default|SetGrowing true))))
    (else
      (Sprite|SetSpriteColor _cue_2 (Math|Color|MakeColor _r _g _b (- _a_2 (/ 0.025 (Variables|Default|GetDifficulty))))))))

(fn ConstructionScript)