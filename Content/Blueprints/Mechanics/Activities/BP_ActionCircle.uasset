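; Action circle actor that runs timed overworld minigames for scavenging, punching, fishing and digging, chosen by the player's ActionState.
; StartActivity spawns that minigame's helper actor, and Activated scores presses by bar fill, circle size, cue opacity or projectile alignment.
; Score narrows a random roll against RewardPercents to pick a RewardPool item for the player's inventory.
; Finished activities return the player to Overworld and destroy the actor.
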(event Custom|Activated
  (bind _circle (Variables|Default|GetCircle))
  ;[1 0 0] Input Action
  (if (Variables|Default|GetActiveAction)
    (Transformation|SetWorldScale3D _circle "0.320000,1.000000,0.320000")
    (Sprite|SetSpriteColor _circle "(R=0.000000,G=0.953125,B=0.126164,A=1.000000)")
    (Utilities|FlowControl|Delay 0.1)
    (Transformation|SetWorldScale3D _circle "0.250000,1.000000,0.250000")
    (Sprite|SetSpriteColor _circle "(R=0.000000,G=0.525490,B=0.670588,A=1.000000)")
    (switch Utilities|FlowControl|Switch|SwitchonENM_ActionState (Variables|/Game/Blueprints/BP_PlayerBase.BP_PlayerBase_C|GetActionState (Variables|Default|GetPlayerReference))
      (:NewEnumerator1
        (CallFunction|ScavengeAction)
        (Audio|PlaySound2D "/Game/Assets/MEchoes/Audio/SFX/DeathHit.DeathHit" 1.0 2.0 0.05 0 0)
        (Utilities|FlowControl|Delay 0.1)
        (Sprite|SetFlipbook (Variables|/Script/Paper2D.PaperCharacter|GetSprite (Variables|Default|GetPlayerReference)) "/Game/Assets/Scum/Flipbooks/FB_ScavengeWait.FB_ScavengeWait"))
      (:NewEnumerator2
        (CallFunction|PunchAction))
      (:NewEnumerator3
        (CallFunction|FishingAction))
      (:NewEnumerator4
        (bind _outputpin (CallFunction|DigAction))
        (Utilities|IsValid _outputpin
          (:Is%20Valid
            (Utilities|FlowControl|DelayUntilNextTick)
            (Actor|DestroyActor _outputpin)
            (Audio|PlaySound2D "/Game/Assets/MEchoes/Audio/SFX/DoubleJumpEffect.DoubleJumpEffect" 2.0 1.0 0.02 0 0)
            (Utilities|FlowControl|Delay 0.1))
          (:Is%20Not%20Valid
            (Utilities|FlowControl|Delay 0.15)))
        (Sprite|SetFlipbook (Variables|/Script/Paper2D.PaperCharacter|GetSprite (Variables|Default|GetPlayerReference)) "/Game/Assets/Scum/Flipbooks/FB_DigWait.FB_DigWait")))))

(event Custom|Start%20Activity
  (bind _returnvalue (Transformation|GetActorTransform))
  (bind _playerreference (Variables|Default|GetPlayerReference))
  (bind _sprite (Variables|/Script/Paper2D.PaperCharacter|GetSprite _playerreference))
  ;[1 0 0] Start Activity
  (Variables|Default|SetActiveAction true)
  (Utilities|FlowControl|DelayUntilNextTick)
  (switch Utilities|FlowControl|Switch|SwitchonENM_ActionState (Variables|/Game/Blueprints/BP_PlayerBase.BP_PlayerBase_C|GetActionState (Variables|Default|GetPlayerReference))
    (:NewEnumerator1
      (Sprite|SetFlipbook _sprite "/Game/Assets/Scum/Flipbooks/FB_ScavengeWait.FB_ScavengeWait")
      ;[0 1 1] Scavenging
      (bind _returnvalue_2 (Game|SpawnActorfromClass "/Game/Blueprints/Mechanics/Activities/BP_ScavengeBar.BP_ScavengeBar_C" _returnvalue "Undefined" "MultiplyWithRoot" 0 0))
      (Variables|Default|SetScavengeBar _returnvalue_2)
      (Utilities|FlowControl|Delay 5.0)
      (Variables|Default|SetActiveAction false)
      (bind _output_get (Variables|Default|SetScore (* (.X (Math|Vector|BreakVector (Variables|/Script/Engine.SceneComponent|GetRelativeScale3D (Variables|/Game/Blueprints/Mechanics/Activities/BP_ScavengeBar.BP_ScavengeBar_C|GetBar (Variables|Default|GetScavengeBar))))) 1e+02)))
      (Development|PrintString (Utilities|String|ToString(Float) _output_get))
      (CallFunction|GiveReward)
      (Utilities|FlowControl|DelayUntilNextTick)
      (Utilities|FlowControl|DelayUntilNextTick)
      (Actor|DestroyActor (Variables|Default|GetScavengeBar))
      (Variables|/Game/Blueprints/BP_PlayerBase.BP_PlayerBase_C|SetActionState (Variables|Default|GetPlayerReference) "NewEnumerator0")
      (Utilities|FlowControl|DelayUntilNextTick)
      (Actor|DestroyActor))
    (:NewEnumerator2
      (Sprite|SetFlipbook _sprite "/Game/Assets/Scum/Flipbooks/FB_PunchPrep.FB_PunchPrep")
      ;[0 1 0] Punching
      (Utilities|FlowControl|Delay 0.2)
      (bind _returnvalue_3 (Game|SpawnActorfromClass "/Game/Blueprints/Mechanics/Activities/BP_PunchCircle.BP_PunchCircle_C" _returnvalue "Undefined" "MultiplyWithRoot" 0 0))
      (bind _output_get_2 (Variables|Default|SetPunchCircle _returnvalue_3))
      (Variables|/Game/Blueprints/Mechanics/Activities/BP_PunchCircle.BP_PunchCircle_C|SetDifficulty _output_get_2 (Variables|Default|GetDifficulty))
      (Variables|/Game/Blueprints/Mechanics/Activities/BP_PunchCircle.BP_PunchCircle_C|SetParentAction _output_get_2 self)
      (Transformation|AddWorldOffset (Variables|/Game/Blueprints/Mechanics/Activities/BP_PunchCircle.BP_PunchCircle_C|GetCircle _output_get_2) "0.000000,1.000000,0.000000" false true))
    (:NewEnumerator3
      (Sprite|SetFlipbook _sprite "/Game/Assets/Scum/Flipbooks/FB_Fishing.FB_Fishing")
      ;[0 0 1] Fishing
      (bind _returnvalue_4 (Game|SpawnActorfromClass "/Game/Blueprints/Mechanics/Activities/BP_FishingCue.BP_FishingCue_C" _returnvalue "Undefined" "MultiplyWithRoot" 0 0))
      (bind _output_get_3 (Variables|Default|SetFishingCue _returnvalue_4))
      (Variables|/Game/Blueprints/Mechanics/Activities/BP_FishingCue.BP_FishingCue_C|SetDifficulty _output_get_3 (Variables|Default|GetDifficulty))
      (Variables|/Game/Blueprints/Mechanics/Activities/BP_FishingCue.BP_FishingCue_C|SetParent%20Action _output_get_3 self)
      (Transformation|AddWorldOffset (Variables|/Game/Blueprints/Mechanics/Activities/BP_FishingCue.BP_FishingCue_C|GetCue _output_get_3) "0.000000,-3.000000,0.000000" false true))
    (:NewEnumerator4
      (Sprite|SetFlipbook _sprite "/Game/Assets/Scum/Flipbooks/FB_DigWait.FB_DigWait")
      ;[1 0 0.5] Digging
      (bind _returnvalue_5 (Utilities|Time|SetTimerbyEvent (delegate Custom|Spawn%20Dig) (* (Variables|Default|GetDifficulty) 2.0) true))
      (CallFunction|SpawnDig)
      (Variables|Default|SetScore 0.0))))

(event Custom|Finish%20Punch
  (bind _punchcircle (Variables|Default|GetPunchCircle))
  (bind _circle (Variables|/Game/Blueprints/Mechanics/Activities/BP_PunchCircle.BP_PunchCircle_C|GetCircle _punchcircle))
  (bind _relativescale3d (Variables|/Script/Engine.SceneComponent|GetRelativeScale3D _circle))
  (bind _x (Math|Vector|BreakVector _relativescale3d))
  (bind _returnvalue (/ 0.23 _x))
  (bind _returnvalue_2 (* _returnvalue 1e+02))
  ;[0 1 0] Punching
  (Variables|Default|SetActiveAction false)
  (Audio|PlaySound2D "/Game/Assets/MEchoes/Audio/SFX/DeathEffect.DeathEffect" 1.2 1.0 0.0 0 0)
  (if (> _returnvalue_2 1.1e+02)
    (bind _output_get (Variables|Default|SetScore (- 1e+02 (- _returnvalue_2 1e+02))))
    (Development|PrintString (Utilities|String|ToString(Float) _output_get))
    (else
      (bind _output_get_2 (Variables|Default|SetScore _returnvalue_2))
      (Development|PrintString (Utilities|String|ToString(Float) _output_get_2))))
  (Utilities|FlowControl|Delay 1.5)
  (CallFunction|GiveReward)
  (Utilities|FlowControl|DelayUntilNextTick)
  (Utilities|FlowControl|DelayUntilNextTick)
  (Actor|DestroyActor (Variables|Default|GetPunchCircle))
  (Variables|/Game/Blueprints/BP_PlayerBase.BP_PlayerBase_C|SetActionState (Variables|Default|GetPlayerReference) "NewEnumerator0")
  (Utilities|FlowControl|DelayUntilNextTick)
  (Actor|DestroyActor))

(event Custom|Finish%20Fishing
  (params (GotFish :type Boolean))
  (bind _fishingcue (Variables|Default|GetFishingCue))
  (bind _cue (Variables|/Game/Blueprints/Mechanics/Activities/BP_FishingCue.BP_FishingCue_C|GetCue _fishingcue))
  (bind _spritecolor (Variables|/Script/Paper2D.PaperSpriteComponent|GetSpriteColor _cue))
  (bind _a (Math|Color|BreakColor _spritecolor))
  (bind _returnvalue (* _a 1e+02))
  (bind _returnvalue_2 (+ _returnvalue 4e+01))
  ;[0 0 1] Fishing
  (Variables|Default|SetActiveAction false)
  (if GotFish
    (if (> _returnvalue_2 0.0)
      (Audio|PlaySound2D "/Game/Assets/Scum/Audio/SFX/ActivityDingAlt.ActivityDingAlt" 1.2 0.5 0.0 0 0)
      (bind _output_get (Variables|Default|SetScore _returnvalue_2))
      (Development|PrintString (Utilities|String|ToString(Float) _output_get))
      (Utilities|FlowControl|Delay 1.5)
      (CallFunction|GiveReward)
      (Utilities|FlowControl|DelayUntilNextTick))
    (else
      (Utilities|FlowControl|Delay 1.0)))
  (Utilities|FlowControl|DelayUntilNextTick)
  (Actor|DestroyActor (Variables|Default|GetFishingCue))
  (Variables|/Game/Blueprints/BP_PlayerBase.BP_PlayerBase_C|SetActionState (Variables|Default|GetPlayerReference) "NewEnumerator0")
  (Utilities|FlowControl|DelayUntilNextTick)
  (Actor|DestroyActor))

(event Custom|Spawn%20Dig
  (bind _spawnpoint (Variables|Default|GetSpawnPoint))
  (bind _returnvalue (Transformation|GetWorldTransform _spawnpoint))
  (bind (_location _rotation) (Math|Transform|BreakTransform _returnvalue))
  ;[1 0 0.5] Digging
  (Development|PrintString "Spawning")
  (bind _returnvalue_2 (Game|SpawnActorfromClass "/Game/Blueprints/Mechanics/BulletLogic/BP_BulletBase.BP_BulletBase_C" (Math|Transform|MakeTransform _location _rotation "0.300000,1.000000,0.300000") "Undefined" "MultiplyWithRoot" 0 0))
  (Variables|/Game/Blueprints/Mechanics/BulletLogic/BP_BulletBase.BP_BulletBase_C|SetSpeed _returnvalue_2 (Variables|Default|GetDifficulty))
  (bind _result (Math|Integer|IncrementInt (Variables|Default|GetCounter))
    (:%20%20
      (if (not (<= _result 4))
        (Utilities|Time|PauseTimerbyHandle (stale Custom|Start%20Activity _returnvalue_5))
        (Utilities|FlowControl|Delay 2.0)
        (bind _output_get (Variables|Default|SetScore (/ (Variables|Default|GetScore) 5.0)))
        (Development|PrintString (Utilities|String|ToString(Float) _output_get))
        (if (>= _output_get 9e+01)
          (Variables|Default|SetScore 1e+02))
        (CallFunction|GiveReward)
        (Utilities|FlowControl|DelayUntilNextTick)
        (Variables|/Game/Blueprints/BP_PlayerBase.BP_PlayerBase_C|SetActionState (Variables|Default|GetPlayerReference) "NewEnumerator0")
        (Utilities|FlowControl|DelayUntilNextTick)
        (Actor|DestroyActor)))))

(fn ConstructionScript)

(fn GiveReward
  (bind _playerreference (Variables|Default|GetPlayerReference))
  (Variables|Default|SetRewarded false)
  (if (< (Variables|Default|GetScore) 1e+01)
    ;[0 1 0.9618] Yield Lowest Reward
    (Variables|Default|SetPrizeNumber 100)
    (else
      ;[0 1 1] Yield Highest Odds
      (if (>= (Variables|Default|GetScore) (Variables|Default|GetBestOdds))
        (Variables|Default|SetScore (Variables|Default|GetBestOdds)))
      (Variables|Default|SetPrizeNumber (Math|Float|Truncate (Math|Random|RandomFloatinRange 0.0 (- 1e+02 (Variables|Default|GetScore)))))))
  (bind (_arrayindex _arrayelement) (Utilities|Array|ReverseforEachLoop (Variables|Default|GetRewardPercents))
    (:LoopBody
      (if (>= _arrayelement (Variables|Default|GetPrizeNumber))
        (if (not (Variables|Default|GetRewarded))
          (Development|PrintString (Utilities|String|Append (Utilities|String|ToString(Integer) _arrayelement) " is greater than" (Utilities|String|ToString(Integer) (Variables|Default|GetPrizeNumber))))
          (Variables|Default|SetSelected _arrayindex)
          (Variables|Default|SetRewarded true))))
    (:Completed
      (bind _returnvalue (Game|SpawnActorfromClass (Utilities|Array|Get(acopy) (Variables|Default|GetRewardPool) (Variables|Default|GetSelected)) (Math|Transform|MakeTransform "0, 0, 0") "Undefined" "MultiplyWithRoot" 0 0))
      (Default|AddItem (Variables|/Game/Blueprints/BP_PlayerBase.BP_PlayerBase_C|GetItemInventory _playerreference) _returnvalue)
      (Default|ItemGetMessage _playerreference _returnvalue)
      (return _returnvalue))))

(fn ScavengeAction
  (bind _scavengebar (Variables|Default|GetScavengeBar))
  (bind _bar (Variables|/Game/Blueprints/Mechanics/Activities/BP_ScavengeBar.BP_ScavengeBar_C|GetBar _scavengebar))
  (bind _relativescale3d (Variables|/Script/Engine.SceneComponent|GetRelativeScale3D _bar))
  (bind (_x _y _z) (Math|Vector|BreakVector _relativescale3d))
  (Sprite|SetFlipbook (Variables|/Script/Paper2D.PaperCharacter|GetSprite (Variables|Default|GetPlayerReference)) "/Game/Assets/Scum/Flipbooks/FB_ScavengeAct.FB_ScavengeAct")
  (Utilities|IsValid _scavengebar
    (:Is%20Valid
      (Transformation|SetRelativeScale3D _bar (Math|Vector|MakeVector (+ _x (* 0.1 (Variables|Default|GetDifficulty))) _y _z)))))

(fn PunchAction
  (bind _punchcircle (Variables|Default|GetPunchCircle))
  (Sprite|SetFlipbook (Variables|/Script/Paper2D.PaperCharacter|GetSprite (Variables|Default|GetPlayerReference)) "/Game/Assets/Scum/Flipbooks/FB_PunchHit.FB_PunchHit")
  (Utilities|IsValid _punchcircle
    (:Is%20Valid
      (CallFunction|FinishPunch)
      (Variables|/Game/Blueprints/Mechanics/Activities/BP_PunchCircle.BP_PunchCircle_C|SetGrowing _punchcircle true)
      (Sprite|SetSpriteColor (Variables|/Game/Blueprints/Mechanics/Activities/BP_PunchCircle.BP_PunchCircle_C|GetCircle _punchcircle) (Math|Color|MakeColor 0.0 1.0 1.0)))))

(fn FishingAction
  (bind _fishingcue (Variables|Default|GetFishingCue))
  (bind _cue (Variables|/Game/Blueprints/Mechanics/Activities/BP_FishingCue.BP_FishingCue_C|GetCue _fishingcue))
  (Sprite|SetFlipbook (Variables|/Script/Paper2D.PaperCharacter|GetSprite (Variables|Default|GetPlayerReference)) "/Game/Assets/Scum/Flipbooks/FB_FishGot.FB_FishGot")
  (Utilities|IsValid _fishingcue
    (:Is%20Valid
      (if (Variables|/Game/Blueprints/Mechanics/Activities/BP_FishingCue.BP_FishingCue_C|GetWaiting _fishingcue)
        (Sprite|SetSpriteColor _cue "(R=1.000000,G=0.052083,B=0.052083,A=1.000000)")
        (Variables|/Game/Blueprints/Mechanics/Activities/BP_FishingCue.BP_FishingCue_C|SetWaiting (Variables|Default|GetFishingCue) false)
        (CallFunction|FinishFishing false)
        (else
          (Actor|Tick|SetActorTickEnabled _fishingcue true)
          (Sprite|SetSpriteColor _cue (Math|Color|MakeColor 0.0 1.0 0.0 (.A (Math|Color|BreakColor (Variables|/Script/Paper2D.PaperSpriteComponent|GetSpriteColor _cue)))))
          (CallFunction|FinishFishing true))))))

(fn DigAction
  (bind _returnvalue (Transformation|GetActorTransform))
  (bind _sphere (Variables|Default|GetSphere))
  (bind _overlappingactors (Collision|GetOverlappingActors _sphere "/Game/Blueprints/Mechanics/BulletLogic/BP_BulletBase.BP_BulletBase_C" :!class /Script/Engine.PrimitiveComponent))
  (bind _location (Math|Transform|BreakTransform _returnvalue))
  (bind _x (Math|Vector|BreakVector _location))
  (bind _output (Utilities|Array|Get(acopy) _overlappingactors))
  (bind _returnvalue_2 (Transformation|GetActorTransform _output))
  (bind _location_2 (Math|Transform|BreakTransform _returnvalue_2))
  (bind _x_2 (Math|Vector|BreakVector _location_2))
  (bind _returnvalue_3 (- _x _x_2))
  (bind _returnvalue_4 (Math|Float|Absolute(Float) _returnvalue_3))
  (Sprite|SetFlipbook (Variables|/Script/Paper2D.PaperCharacter|GetSprite (Variables|Default|GetPlayerReference)) "/Game/Assets/Scum/Flipbooks/FB_DigPull.FB_DigPull")
  (Utilities|IsValid _output
    (:Is%20Valid
      (Development|PrintString (Utilities|String|ToString(Float) _returnvalue_4))
      (if (<= _returnvalue_4 1e+02)
        (Variables|Default|SetScore (+ (- 1e+02 _returnvalue_4) (Variables|Default|GetScore))))
      (return _output))
    (:Is%20Not%20Valid
      (return 0))))