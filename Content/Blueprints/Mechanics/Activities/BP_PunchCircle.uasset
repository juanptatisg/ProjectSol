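; BP_PunchCircle is a sprite circle visual for a punch activity, animated as either a shrinking or an expanding ring.
; By default Tick shrinks the Circle's X and Z scale at a rate inversely proportional to Difficulty while fading it in, then hides it and stops ticking at zero.
; When Growing is set, which this graph never does, it expands and fades out instead.
; All steps are fixed per frame, independent of delta time.
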(event EventBeginPlay
  (Sprite|SetSpriteColor (Variables|Default|GetCircle) (Math|Color|MakeColor 0.8 0.0 1.0 0.0)))

(event EventTick
  (params (DeltaSeconds :type Float%20%28single-precision%29))
  (bind _circle (Variables|Default|GetCircle))
  (bind _difficulty (Variables|Default|GetDifficulty))
  (bind _circle_2 (Variables|Default|GetCircle))
  (bind _circle_3 (Variables|Default|GetCircle))
  (bind _returnvalue (/ 0.01 _difficulty))
  (bind _relativescale3d (Variables|/Script/Engine.SceneComponent|GetRelativeScale3D _circle_3))
  (bind _spritecolor (Variables|/Script/Paper2D.PaperSpriteComponent|GetSpriteColor _circle_2))
  (bind _relativescale3d_2 (Variables|/Script/Engine.SceneComponent|GetRelativeScale3D _circle))
  (bind (_x _y) (Math|Vector|BreakVector _relativescale3d))
  (bind (_r _g _b _a) (Math|Color|BreakColor _spritecolor))
  (bind (_x_2 _y_2) (Math|Vector|BreakVector _relativescale3d_2))
  (bind _returnvalue_2 (- _x _returnvalue))
  (bind _returnvalue_3 (+ _x_2 0.07))
  (if (Variables|Default|GetGrowing)
    (Transformation|SetRelativeScale3D _circle (Math|Vector|MakeVector _returnvalue_3 _y_2 _returnvalue_3))
    (Sprite|SetSpriteColor _circle_2 (Math|Color|MakeColor _r _g _b (- _a 0.1)))
    (else
      (Transformation|SetRelativeScale3D _circle_3 (Math|Vector|MakeVector _returnvalue_2 _y _returnvalue_2))
      (if (> (.X (Math|Vector|BreakVector (Variables|/Script/Engine.SceneComponent|GetRelativeScale3D _circle_3))) 0.0)
        (Sprite|SetSpriteColor (Variables|Default|GetCircle) (Math|Color|MakeColor 0.8 0.0 1.0 (+ (.A (Math|Color|BreakColor (Variables|/Script/Paper2D.PaperSpriteComponent|GetSpriteColor (Variables|Default|GetCircle)))) 0.1)))
        (else
          (Actor|Tick|SetActorTickEnabled false)
          (Sprite|SetSpriteColor (Variables|Default|GetCircle) (Math|Color|MakeColor 0.0 0.0 0.0 0.0)))))))

(fn ConstructionScript)