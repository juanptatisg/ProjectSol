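; BP_ScavengeBar is a depleting bar indicator, named for the scavenge activity, built from Bar and Circle sprites.
; Each tick shrinks the Bar's X scale by a fixed step, independent of delta time, and clamps it at zero.
; The remaining X scale drives a semi-transparent green-to-red tint on both sprites as the bar empties.
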(event EventTick
  (params (DeltaSeconds :type Float%20%28single-precision%29))
  (bind _bar (Variables|Default|GetBar))
  (bind _bar_2 (Variables|Default|GetBar))
  (bind _relativescale3d (Variables|/Script/Engine.SceneComponent|GetRelativeScale3D _bar))
  (bind _relativescale3d_2 (Variables|/Script/Engine.SceneComponent|GetRelativeScale3D _bar_2))
  (bind _x (Math|Vector|BreakVector _relativescale3d))
  (bind (_x_2 _y _z) (Math|Vector|BreakVector _relativescale3d_2))
  (bind _returnvalue (- 1.0 _x))
  (bind _returnvalue_2 (Math|Color|MakeColor _returnvalue _x 0.0 0.5))
  (Transformation|SetRelativeScale3D _bar_2 (Math|Vector|MakeVector (- _x_2 0.025) _y _z))
  (if (> (.X (Math|Vector|BreakVector (Variables|/Script/Engine.SceneComponent|GetRelativeScale3D (Variables|Default|GetBar)))) 0.0)
    _
    (else
      (Transformation|SetRelativeScale3D _bar "0.000000,1.000000,0.100000")))
  (Sprite|SetSpriteColor (Variables|Default|GetBar) _returnvalue_2)
  (Sprite|SetSpriteColor (Variables|Default|GetCircle) _returnvalue_2))

(fn ConstructionScript)