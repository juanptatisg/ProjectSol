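; Base overworld player character: a Paper2D sprite in 3D space with movement, interaction, inventory and pause controls.
; BeginPlay spawns a linked BP_PlayerBattler with hardcoded stats and the quest overlay; the loaded save is unused.
; Tick selects flipbooks from velocity and mirrors the sprite and camera offset, while an occluder box fades overlapping world sprites.
; Interact, routed by ActionState, starts cutscenes, collects items or triggers action circles; equipment modifiers sum onto the battler.
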(event OnComponentBeginOverlap(OccluderBox)
  (params (OverlappedComponent :type Primitive%20Component%20Object%20Reference) (OtherActor :type Actor%20Object%20Reference) (OtherComp :type Primitive%20Component%20Object%20Reference) (OtherBodyIndex :type Integer) (bFromSweep :type Boolean) (SweepResult :type Hit%20Result%20Structure%20%28by%20ref%29))
  ;[0 1 0.9659] Occluding Sprites near camera
  (if (Actor|ActorHasTag OtherActor "WorldSprite")
    (Development|PrintString "make invis")
    (bind _aspaper_sprite_component (Utilities|Casting|CastToPaperSpriteComponent OtherComp))
    (bind _alpha (Timeline|MakeTransparent PlayFromStart)
      (:Update
        (Sprite|SetSpriteColor _aspaper_sprite_component (Utilities|Struct|MakeLinearColor (.r (Variables|/Script/Paper2D.PaperSpriteComponent|GetSpriteColor _aspaper_sprite_component)) (.g (Variables|/Script/Paper2D.PaperSpriteComponent|GetSpriteColor _aspaper_sprite_component)) (.b (Variables|/Script/Paper2D.PaperSpriteComponent|GetSpriteColor _aspaper_sprite_component)) _alpha)))
      (:Finished
        (Sprite|SetSpriteColor _aspaper_sprite_component (Utilities|Struct|MakeLinearColor (.r (Variables|/Script/Paper2D.PaperSpriteComponent|GetSpriteColor _aspaper_sprite_component)) (.g (Variables|/Script/Paper2D.PaperSpriteComponent|GetSpriteColor _aspaper_sprite_component)) (.b (Variables|/Script/Paper2D.PaperSpriteComponent|GetSpriteColor _aspaper_sprite_component)) 0.2))))))

(event OnComponentEndOverlap(OccluderBox)
  (params (OverlappedComponent :type Primitive%20Component%20Object%20Reference) (OtherActor :type Actor%20Object%20Reference) (OtherComp :type Primitive%20Component%20Object%20Reference) (OtherBodyIndex :type Integer))
  ;[0 1 0.9659] Occluding Sprites near camera
  (if (Actor|ActorHasTag OtherActor "WorldSprite")
    (bind _aspaper_sprite_component (Utilities|Casting|CastToPaperSpriteComponent OtherComp))
    (bind _alpha (Timeline|ReverseTransparent ReverseFromEnd)
      (:Update
        (Sprite|SetSpriteColor _aspaper_sprite_component (Utilities|Struct|MakeLinearColor (.r (Variables|/Script/Paper2D.PaperSpriteComponent|GetSpriteColor _aspaper_sprite_component)) (.g (Variables|/Script/Paper2D.PaperSpriteComponent|GetSpriteColor _aspaper_sprite_component)) (.b (Variables|/Script/Paper2D.PaperSpriteComponent|GetSpriteColor _aspaper_sprite_component)) _alpha))))))

(event Custom|parar
  (bind _camera (Variables|Default|GetCamera))
  ;[1 1 1] Idle Anim base
  (bind _saturation (Timeline|IdleTimeline PlayFromStart)
    (:Update
      (Variables|/Script/Engine.CameraComponent|SetPostProcessSettings _camera (Utilities|Struct|MakePostProcessSettings (Math|Vector4|MakeVector4 (.x (Utilities|Struct|BreakPostProcessSettings (Variables|/Script/Engine.CameraComponent|GetPostProcessSettings _camera))) (.y (Utilities|Struct|BreakPostProcessSettings (Variables|/Script/Engine.CameraComponent|GetPostProcessSettings _camera))) _saturation (.w (Utilities|Struct|BreakPostProcessSettings (Variables|/Script/Engine.CameraComponent|GetPostProcessSettings _camera)))))))))

(event EventBeginPlay
  ;[0.02832 0 1] Startup
  (Utilities|FlowControl|DelayUntilNextTick)
  (bind _returnvalue (Settings|GetGameUserSettings))
  (Class|GameUserSettings|SetVSyncEnabled _returnvalue true)
  (bind _asplayer_controller (Utilities|Casting|CastToPlayerController (Pawn|GetController)))
  (Utilities|IsValid (PlayerController|LocalPlayerSubsystems|GetEnhancedInputLocalPlayerSubsystem _asplayer_controller)
    (:Is%20Valid
      (Input|AddMappingContext (PlayerController|LocalPlayerSubsystems|GetEnhancedInputLocalPlayerSubsystem _asplayer_controller) "/Game/Input/IM_BaseGame.IM_BaseGame" 0 "(bIgnoreAllPressedKeysUntilRelease=True,bForceImmediately=False,bNotifyUserSettings=False)")
      (bind _savegame (|AsyncLoadGamefromSlot "A")
        (:Completed
          (bind _assave_game_1 (Utilities|Casting|CastToSaveGame1 _savegame)
            (:then
              _)
            (:CastFailed
              _))
          ;[0 0.004602 1] Prep Batller
          (bind _returnvalue_2 (Game|SpawnActorfromClass "/Game/Blueprints/BP_PlayerBattler.BP_PlayerBattler_C" (Math|Transform|MakeTransform (Variables|Default|GetCombatLocation)) "Undefined" "MultiplyWithRoot" 0 0))
          (bind _output_get (Variables|Default|SetBattler _returnvalue_2))
          (Variables|/Game/Blueprints/BP_PlayerBattler.BP_PlayerBattler_C|SetOverworldPlayer _output_get self)
          (Default|UpdateStats _output_get (Utilities|Struct|MakeST_Stats 1 2e+02 1e+02 2e+01 2e+01 5.0 0.05 1.0))
          (bind _returnvalue_3 (UserInterface|CreateWidget "/Game/Blueprints/UI/WBP_QuestOverlay.WBP_QuestOverlay_C" 0 (Variables|Default|GetBP_QuestComponent)))
          (UserInterface|Viewport|AddtoViewport _returnvalue_3 0)
          (Variables|/Game/Blueprints/UI/WBP_QuestOverlay.WBP_QuestOverlay_C|SetBattlerRef _returnvalue_3 (Variables|Default|GetBattler)))))))

(event EventTick
  (params (DeltaSeconds :type Float%20%28single-precision%29))
  (Utilities|FlowControl|Sequence
    (:then_0
      (CallFunction|UpdateFlipbook))
    (:then_1
      (CallFunction|UpdatePlayerRotation))))

(event Collision|EventActorBeginOverlap
  (params (OtherActor :type Actor%20Object%20Reference))
  ;[1 1 1] Overlap Event for Camera Bounds
)

(event Collision|EventActorEndOverlap
  (params (OtherActor :type Actor%20Object%20Reference))
  ;[1 1 1] Indicate Player has left all Camera Bounds
)

(event Input|KeyboardEvents|6
  (params (Key :type Key%20Structure :default "None"))
  ;[1 1 1] Idle Anim base
  (:Pressed
    (if true
      (bind _returnvalue (Utilities|Time|SetTimerbyEvent (delegate Custom|parar) 5.0))
      (Variables|Default|SetIdleTimer _returnvalue))))

(event Input|KeyboardEvents|7
  (params (Key :type Key%20Structure :default "None"))
  (bind _idletimer (Variables|Default|GetIdleTimer))
  ;[1 1 1] Idle Anim base
  (:Pressed
    (if (Utilities|Time|IsValidTimerHandle _idletimer)
      (Utilities|Time|ClearandInvalidateTimerbyHandle _idletimer))))

(event Input|EnhancedActionEvents|EnhancedInputActionIA_MoveRight
  (params (ActionValue :type Float%20%28double-precision%29) (ElapsedSeconds :type Float%20%28double-precision%29) (TriggeredSeconds :type Float%20%28double-precision%29) (InputAction :type Input%20Action%20Object%20Reference :default "/Game/Input/IA_MoveRight.IA_MoveRight"))
  ;[1 0 0] Directional Movement
  (if (Utilities|Enum|Equal(Enum) (Variables|Default|GetActionState) "NewEnumerator0")
    (bind _output_get (Variables|Default|SetCurrentDirection ActionValue))
    (Pawn|Input|AddMovementInput "1.000000,0.000000,0.000000" _output_get false)))

(event Input|EnhancedActionEvents|EnhancedInputActionIA_MoveUp
  (params (ActionValue :type Float%20%28double-precision%29) (ElapsedSeconds :type Float%20%28double-precision%29) (TriggeredSeconds :type Float%20%28double-precision%29) (InputAction :type Input%20Action%20Object%20Reference :default "/Game/Input/IA_MoveUp.IA_MoveUp"))
  ;[1 0 0] Directional Movement
  (if (Utilities|Enum|Equal(Enum) (Variables|Default|GetActionState) "NewEnumerator0")
    (Pawn|Input|AddMovementInput "0.000000,-1.000000,0.000000" ActionValue false)))

(event Input|ActionEvents|InputActionPause
  (params (Key :type Key%20Structure :default "None"))
  ;[1 0.005208 0.005208] Pause
  (:Pressed
    (Utilities|IsValid (Variables|Default|GetPauseReference)
      (:Is%20Valid
        _)
      (:Is%20Not%20Valid
        (bind _returnvalue (UserInterface|CreateWidget "/Game/Blueprints/UI/PauseMenu/PauseMenu.PauseMenu_C"))
        (Variables|Default|SetPauseReference _returnvalue)))
    (Variables|/Script/Engine.PlayerController|SetbShowMouseCursor (Game|GetPlayerController 0) true)
    (UserInterface|Viewport|AddtoViewport (Variables|Default|GetPauseReference) 0)
    (bind _returnvalue_2 (Game|SetGamePaused true))
    (Variables|/Game/Blueprints/UI/PauseMenu/PauseMenu.PauseMenu_C|SetPaused (Variables|Default|GetPauseReference) _returnvalue_2)))

(event Input|ActionEvents|InputActionWalk
  (params (Key :type Key%20Structure :default "None"))
  ;[1 0 0] Footsteps Sound
  (:Pressed
    (Variables|Default|SetWalking true)
    (if (Variables|Default|GetWalking) :!label _label
      (Utilities|FlowControl|Delay 0.35)
      (Utilities|FlowControl|Sequence
        (:then_0
          (if (Pawn|Components|CharacterMovement|IsWalking (Variables|Character|GetCharacterMovement))
            (if (Utilities|Array|IsEmpty (Collision|GetOverlappingActors "/Game/Assets/Scum/Textures/Agua_Blueprint.Agua_Blueprint_C" :!class /Script/Engine.Actor))
              (Audio|PlaySound2D "/Game/Assets/MEchoes/Audio/SFX/Step_SFX.Step_SFX" 1.0 1.0 0.0 0 0 false)
              (else
                (Development|PrintString "agua")
                (Audio|PlaySound2D "/Game/Assets/Scum/Audio/SFX/cartoon_waterdrop-37499.cartoon_waterdrop-37499" 0.3 1.5 0.0 0 0)))))
        (:then_1
          (goto _label)))))
  (:Released
    (Variables|Default|SetWalking false)))

(event Input|ActionEvents|InputActionInteract
  (params (Key :type Key%20Structure :default "None"))
  (bind _returnvalue (Game|GetPlayerController 0))
  (bind _returnvalue_2 (Game|GetPlayerController 0))
  (bind _statuswidget (Variables|Default|GetStatusWidget))
  (bind _actioncircle (Variables|Default|GetActionCircle))
  (bind _wbp_items (Variables|/Game/Blueprints/UI/StatusMenu/WB_GeneralMenu.WB_GeneralMenu_C|GetWBP_Items _statuswidget))
  (:Pressed
    (switch Utilities|FlowControl|Switch|SwitchonENM_ActionState (Variables|Default|GetActionState)
      (:NewEnumerator0
        (Utilities|FlowControl|DelayUntilNextTick)
        (if (not (Variables|Default|GetInvOpen))
          (if (Variables|Default|GetInsideCutscene)
            (Utilities|IsValid (Variables|Default|GetCutsceneReference)
              (:Is%20Valid
                ;[1 0 0] Activate TextCutscene
                (Audio|PlaySound2D "/Game/Assets/MEchoes/Audio/SFX/UI_Ding.UI_Ding" 1.2 1.0 0.0 0 0)
                (Input|DisableInput _returnvalue_2)
                (Utilities|FlowControl|DelayUntilNextTick)
                (bind _returnvalue_3 (UserInterface|CreateWidget "/Game/Blueprints/Mechanics/DialogueSystem/UI/TextCutscene.TextCutscene_C" _returnvalue_2))
                (UserInterface|Viewport|AddtoViewport _returnvalue_3 0)
                (Variables|/Game/Blueprints/Mechanics/DialogueSystem/UI/TextCutscene.TextCutscene_C|SetEventData _returnvalue_3 (Variables|/Game/Blueprints/Interactives/Technical/CutsceneControl.CutsceneControl_C|GetSceneData (Variables|Default|GetCutsceneReference)))
                (Variables|/Game/Blueprints/Mechanics/DialogueSystem/UI/TextCutscene.TextCutscene_C|SetPlayerCharacter _returnvalue_3 self)
                (Rendering|SetVisibility (Variables|Default|GetThoughtBubble) false false)
                (Variables|Default|SetInsideCutscene false)
                (if (Variables|/Game/Blueprints/Interactives/Technical/CutsceneControl.CutsceneControl_C|GetFaceRight (Variables|Default|GetCutsceneReference))
                  (Pawn|SetControlRotation _returnvalue (Math|Rotator|MakeRotator 0.0 0.0 0.0))
                  (else
                    (Pawn|SetControlRotation _returnvalue (Math|Rotator|MakeRotator 0.0 0.0 1.8e+02))))))
            (else
              ;[0 1 0.9743] Pick Up Item
              (for _array_element (Collision|GetOverlappingActors "/Game/Blueprints/Mechanics/BP_Item.BP_Item_C" :!class /Script/Engine.Actor)
                (if (Utilities|DoesObjectImplementInterface _array_element "/Game/Blueprints/Mechanics/Inventory/BPI_PickUpItem.BPI_PickUpItem_C")
                  (bind _item (Class|BPIPickUpItem|PickUp(Message) _array_element))
                  (Utilities|FlowControl|Sequence
                    (:then_0
                      (Utilities|IsValid _statuswidget
                        (:Is%20Valid
                          (switch Utilities|FlowControl|Switch|SwitchonENM_ItemType (Variables|/Game/Blueprints/Mechanics/BP_Item.BP_Item_C|GetItemType _item)
                            (:NewEnumerator0
                              (Default|AddCollectable _wbp_items _item))
                            (:NewEnumerator1
                              (Default|AddKey _wbp_items _item))
                            (:NewEnumerator2
                              (Default|AddAccessory (Variables|/Game/Blueprints/UI/StatusMenu/WB_GeneralMenu.WB_GeneralMenu_C|GetWBP_Equip _statuswidget) _item))))
                        (:Is%20Not%20Valid
                          _))
                      (CallFunction|ItemGetMessage _item))
                    (:then_1
                      (Default|AddItem (Utilities|Select :Index (Variables|/Game/Blueprints/Mechanics/BP_Item.BP_Item_C|GetItemType _item) :NewEnumerator0 (Variables|Default|GetCollectableInventory) :NewEnumerator1 (Variables|Default|GetKeyItemInventory) :NewEnumerator2 (Variables|Default|GetAccessoryInventory)) _item)
                      (Utilities|FlowControl|DelayUntilNextTick)
                      (Actor|DestroyActor _array_element)))))))))
      (:NewEnumerator1
        (Utilities|IsValid _actioncircle :!label _label
          (:Is%20Valid
            (Default|Activated _actioncircle))))
      (:NewEnumerator2
        (goto _label))
      (:NewEnumerator3
        (goto _label))
      (:NewEnumerator4
        (goto _label)))))

(event Input|KeyboardEvents|1
  (params (Key :type Key%20Structure :default "None"))
  (:Pressed
    (Default|LevelUp (Variables|Default|GetBattler))))

(event Input|KeyboardEvents|Q
  (params (Key :type Key%20Structure :default "None"))
  (bind _returnvalue (Game|GetPlayerController 0))
  (:Pressed
    (if (Utilities|Enum|Equal(Enum) (Variables|Default|GetActionState) "NewEnumerator0")
      ;[1 0.9197 0] Opne/Close inventory
      (Utilities|FlowControl|FlipFlop
        (:A
          (bind _statuswidget (Variables|Default|GetStatusWidget)
            (:then
              (Variables|/Script/UMG.Widget|SetVisibility _statuswidget "Visible"))
            (:else
              (bind _returnvalue_2 (UserInterface|CreateWidget "/Game/Blueprints/UI/StatusMenu/WB_GeneralMenu.WB_GeneralMenu_C" (Game|GetPlayerController 0)))
              (bind _output_get (Variables|Default|SetStatusWidget _returnvalue_2))
              (Variables|/Game/Blueprints/UI/StatusMenu/WB_GeneralMenu.WB_GeneralMenu_C|SetPlayer _output_get self)
              (UserInterface|Viewport|AddtoViewport _output_get 0)))
          (Variables|Default|SetInvOpen true)
          (Input|SetInputModeGameandUI _returnvalue 0 "DoNotLock" true false)
          (Variables|/Script/Engine.PlayerController|SetbShowMouseCursor _returnvalue true))
        (:B
          (bind _statuswidget_2 (Variables|Default|GetStatusWidget)
            (:then
              (if (Variables|Default|GetInvOpen)
                (Variables|/Script/UMG.Widget|SetVisibility _statuswidget_2 "Hidden")
                (Variables|Default|SetInvOpen false)
                (Input|SetInputModeGameOnly _returnvalue false)
                (Variables|/Script/Engine.PlayerController|SetbShowMouseCursor _returnvalue false)))
            (:else)))))))

(fn ConstructionScript)

(fn UpdateFlipbook
  (if (Utilities|Enum|Equal(Enum) (Variables|Default|GetActionState) "NewEnumerator0")
    (if (Variables|Default|GetDashing)
      (Sprite|SetFlipbook (Variables|Default|GetSprite) (Variables|FB|GetFB_Dash))
      (elif (not false)
        (Variables|Default|SetMovementState (select (!= (Math|Vector|VectorLength (Transformation|GetVelocity)) 0.0) (select (AI|Components|NavMovement|IsFalling (Variables|Character|GetCharacterMovement)) (select (<= (.z (Transformation|GetVelocity)) 0.0) "NewEnumerator4" "NewEnumerator3") "NewEnumerator2") "NewEnumerator1"))
        (Sprite|SetFlipbook (Variables|Default|GetSprite) (Utilities|Select :Index (Variables|Default|GetMovementState) :NewEnumerator0 0 :NewEnumerator1 (Variables|FB|GetFB_Idle) :NewEnumerator2 (Variables|FB|GetFB_Run) :NewEnumerator3 (Variables|FB|GetFB_Jump) :NewEnumerator4 (Variables|FB|GetFB_Fall)))))))

(fn UpdatePlayerRotation
  (bind _springarm (Variables|Default|GetSpringArm))
  (bind _springarm_2 (Variables|Default|GetSpringArm))
  (bind _sprite (Variables|Default|GetSprite))
  (bind _sprite_2 (Variables|Default|GetSprite))
  (bind _relativescale3d (Variables|/Script/Engine.SceneComponent|GetRelativeScale3D _sprite))
  (bind _relativescale3d_2 (Variables|/Script/Engine.SceneComponent|GetRelativeScale3D _sprite_2))
  (Math|Float|CompareFloat (.x (Transformation|GetVelocity)) 0.0
    (:>
      (Transformation|SetRelativeScale3D _sprite_2 (Math|Vector|MakeVector (* (Math|Float|SelectFloat -1.0 1.0 (< (.x _relativescale3d_2) 0.0)) (.x _relativescale3d_2)) (.y _relativescale3d_2) (.z _relativescale3d_2)))
      (Variables|/Script/Engine.SpringArmComponent|SetTargetOffset _springarm (Math|Vector|MakeVector 1.2e+02 (.y (Variables|/Script/Engine.SpringArmComponent|GetTargetOffset _springarm)) (.z (Variables|/Script/Engine.SpringArmComponent|GetTargetOffset _springarm)))))
    (:<
      (Transformation|SetRelativeScale3D _sprite (Math|Vector|MakeVector (* (Math|Float|SelectFloat -1.0 1.0 (> (.x _relativescale3d) 0.0)) (.x _relativescale3d)) (.y _relativescale3d) (.z _relativescale3d)))
      (Variables|/Script/Engine.SpringArmComponent|SetTargetOffset _springarm_2 (Math|Vector|MakeVector -1.2e+02 (.y (Variables|/Script/Engine.SpringArmComponent|GetTargetOffset _springarm_2)) (.z (Variables|/Script/Engine.SpringArmComponent|GetTargetOffset _springarm_2)))))))

(fn CancelMovement
  (Variables|/Script/Engine.MovementComponent|SetVelocity (Variables|Character|GetCharacterMovement) "0, 0, 0")
  (Components|Movement|StopMovementImmediately (Variables|Character|GetCharacterMovement))
  (Class|PrimitiveComponent|SetAllPhysicsLinearVelocity (Variables|Collision|GetCapsuleComponent) "0, 0, 0" false))

(fn ItemGetMessage
  (params (Item :type BP%20Item%20Object%20Reference))
  (bind _returnvalue (Transformation|GetActorTransform))
  (bind _returnvalue_2 (Game|SpawnActorfromClass "/Game/Blueprints/Mechanics/Items/BP_ItemCollectMessage.BP_ItemCollectMessage_C" (Math|Transform|MakeTransform (Math|Vector|MakeVector (.x (.location _returnvalue)) (.y (.location _returnvalue)) (+ (.z (.location _returnvalue)) 215.0)) "0.000000,90.000000,0.000000" (.scale _returnvalue)) "AlwaysSpawn" "MultiplyWithRoot" 0 0))
  (Rendering|Components|TextRender|SetText (Variables|/Game/Blueprints/Mechanics/Items/BP_ItemCollectMessage.BP_ItemCollectMessage_C|GetTextRender _returnvalue_2) (Utilities|Text|ToText(String) (Utilities|String|Append (Variables|/Game/Blueprints/Mechanics/BP_Item.BP_Item_C|GetItemName Item) " x" (Utilities|String|ToString(Integer) (Variables|/Game/Blueprints/Mechanics/BP_Item.BP_Item_C|GetQuantity Item)))))
  (Audio|PlaySound2D "/Game/Assets/MEchoes/Audio/SFX/PowerUnlock.PowerUnlock" 0.9 1.5 0.0 0 0))

(fn ApplyEquipmentStats
  (bind _battler (Variables|Default|GetBattler))
  (Variables|/Game/Blueprints/BP_PlayerBattler.BP_PlayerBattler_C|SetEquipMods (Variables|Default|GetBattler) (Utilities|Struct|MakeST_Stats 0 0.0 0.0 0.0 0.0 0.0 0.0 0.0))
  (for _array_element (Variables|Default|GetEquipmentArray)
    (Variables|/Game/Blueprints/BP_PlayerBattler.BP_PlayerBattler_C|SetEquipMods _battler (Utilities|Struct|MakeST_Stats 0 (+ (.maxhp (Variables|/Game/Blueprints/BP_PlayerBattler.BP_PlayerBattler_C|GetEquipMods _battler)) (.maxhp (Variables|/Game/Blueprints/Mechanics/BP_Item.BP_Item_C|GetItemModifiers _array_element))) (+ (.energy (Variables|/Game/Blueprints/BP_PlayerBattler.BP_PlayerBattler_C|GetEquipMods _battler)) (.energy (Variables|/Game/Blueprints/Mechanics/BP_Item.BP_Item_C|GetItemModifiers _array_element))) (+ (.attack (Variables|/Game/Blueprints/BP_PlayerBattler.BP_PlayerBattler_C|GetEquipMods _battler)) (.attack (Variables|/Game/Blueprints/Mechanics/BP_Item.BP_Item_C|GetItemModifiers _array_element))) (+ (.defense (Variables|/Game/Blueprints/BP_PlayerBattler.BP_PlayerBattler_C|GetEquipMods _battler)) (.defense (Variables|/Game/Blueprints/Mechanics/BP_Item.BP_Item_C|GetItemModifiers _array_element))) (+ (.healing (Variables|/Game/Blueprints/BP_PlayerBattler.BP_PlayerBattler_C|GetEquipMods _battler)) (.healing (Variables|/Game/Blueprints/Mechanics/BP_Item.BP_Item_C|GetItemModifiers _array_element))) (+ (.critrate (Variables|/Game/Blueprints/BP_PlayerBattler.BP_PlayerBattler_C|GetEquipMods _battler)) (.critrate (Variables|/Game/Blueprints/Mechanics/BP_Item.BP_Item_C|GetItemModifiers _array_element))) (+ (.energygain (Variables|/Game/Blueprints/BP_PlayerBattler.BP_PlayerBattler_C|GetEquipMods _battler)) (.energygain (Variables|/Game/Blueprints/Mechanics/BP_Item.BP_Item_C|GetItemModifiers _array_element)))))))