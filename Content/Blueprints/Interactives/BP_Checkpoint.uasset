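; One-shot checkpoint for a 2D Paper2D game that triggers when an actor tagged "Player" first overlaps it.
; On activation it plays a jingle, tints its flipbook purple and teleports the first "Respawn"-tagged actor to its X and Z, with Y zeroed.
; It then asynchronously loads slot "A", writes the player's day index and current level into it, and saves to the slot stored in that save object.
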(event Collision|EventActorBeginOverlap
  (params (OtherActor :type Actor%20Object%20Reference))
  (bind _returnvalue (Transformation|GetActorLocation))
  (bind (_x _y _z) (Class|KismetMathLibrary|BreakVector3f _returnvalue))
  (if (not (Variables|Default|GetUsed))
    (if (Actor|ActorHasTag OtherActor "Player")
      (Utilities|FlowControl|Sequence
        (:then_0
          (Audio|PlaySound2D "/Game/Assets/MEchoes/Audio/SFX/CheckpointJingle__1_.CheckpointJingle__1_" 0.7 1.0 0.0 0 0)
          (Sprite|SetSpriteColor (Variables|Default|GetPaperFlipbook) (Math|Color|MakeColor 0.6 0.2 1.0))
          (Variables|Default|SetUsed true))
        (:then_1
          (bind _outactors (Actor|GetAllActorswithTag "Respawn"))
          (Transformation|SetActorLocation (Utilities|Array|Get(acopy) _outactors) (Math|Vector|MakeVector _x 0.0 _z) false true)
          (bind _savegame (|AsyncLoadGamefromSlot "A")
            (:Completed
              (bind _assave_game_1 (Utilities|Casting|CastToSaveGame1 _savegame))
              (bind _output_get (Variables|Default|SetSaveInstance _assave_game_1))
              (bind _asbp_player_base (Utilities|Casting|CastToBP_PlayerBase OtherActor))
              (Utilities|FlowControl|Sequence
                (:then_0
                  ;[1 1 1] Set All Save Values
                  (Variables|/Game/Blueprints/Saving/SaveGame1.SaveGame1_C|SetDayState _output_get (Variables|/Game/Blueprints/BP_PlayerBase.BP_PlayerBase_C|GetDayIndex _asbp_player_base))
                  (Variables|/Game/Blueprints/Saving/SaveGame1.SaveGame1_C|SetLastLevel _output_get (Variables|Default|GetCurrentLevel)))
                (:then_1
                  (|AsyncSaveGametoSlot _output_get (Variables|/Game/Blueprints/Saving/SaveGame1.SaveGame1_C|GetSlot _output_get) (Variables|/Game/Blueprints/Saving/SaveGame1.SaveGame1_C|GetUserIndex _output_get)))))))))))

(fn ConstructionScript)