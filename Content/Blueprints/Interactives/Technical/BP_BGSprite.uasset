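; BP_BGSprite is a Paper2D sprite Blueprint, named as a background sprite, that can be hidden and shown through FadeOut and FadeIn.
; Each function checks the Invisible flag, steps the PaperSprite's color alpha toward zero or one while preserving RGB, then flips the flag.
; The while loops contain no delay, so each fade completes within a single call rather than animating over frames.
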(fn ConstructionScript)

(fn FadeOut
  (bind _papersprite (Variables|Default|GetPaperSprite))
  (bind _spritecolor (Variables|/Script/Paper2D.PaperSpriteComponent|GetSpriteColor _papersprite))
  (bind (_r _g _b _a) (Math|Color|BreakColor _spritecolor))
  (if (not (Variables|Default|GetInvisible))
    (while (> _a 0.0)
      (Sprite|SetSpriteColor _papersprite (Math|Color|MakeColor _r _g _b (+ _a -0.02))))
    (Variables|Default|SetInvisible true)))

(fn Fadein
  (bind _papersprite (Variables|Default|GetPaperSprite))
  (bind _spritecolor (Variables|/Script/Paper2D.PaperSpriteComponent|GetSpriteColor _papersprite))
  (bind (_r _g _b _a) (Math|Color|BreakColor _spritecolor))
  (if (Variables|Default|GetInvisible)
    (while (< _a 1.0)
      (Sprite|SetSpriteColor _papersprite (Math|Color|MakeColor _r _g _b (+ _a 0.02))))
    (Variables|Default|SetInvisible false)))