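; BP_MusicBox is a trigger actor that starts its assigned OverworldSong when an actor tagged Player overlaps it.
; It stores the song as the OverworldTrack on MusicControl and tells MusicControl to play it.
; ActivationBox then ignores all collision channels, so the trigger fires only once.
; A fade-and-stop chain of LowerVolume, Delay and StopTrack is present but never runs.
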(event Collision|EventActorBeginOverlap
  (params (OtherActor :type Actor%20Object%20Reference))
  (bind _musiccontrol (Variables|Default|GetMusicControl))
  (if (Actor|ActorHasTag OtherActor "Player")
    (bind _output_get (Variables|/Game/Blueprints/Interactives/Technical/BP_MusicControl.BP_MusicControl_C|SetOverworldTrack _musiccontrol (Variables|Default|GetOverworldSong)))
    (Default|PlayTrack _musiccontrol _output_get)
    (Collision|SetCollisionResponsetoAllChannels (Variables|Default|GetActivationBox) "ECR_Ignore")))

(fn ConstructionScript)