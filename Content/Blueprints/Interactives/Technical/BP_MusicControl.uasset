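; BP_MusicControl is a music controller that plays one non-spatialized track at a time through callable functions.
; PlayTrack stops any valid current track, creates a 2D sound from the given song, stores it as Track and plays it.
; StopTrack stops the track and LowerVolume linearly fades it to silence over a few seconds.
; Both act only when the Playing flag is true, which this Blueprint's graphs never set.
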(event EventBeginPlay)

(fn ConstructionScript)

(fn PlayTrack
  (params (Song :type Sound%20Base%20Object%20Reference))
  (Utilities|IsValid (Variables|Default|GetTrack)
    (:Is%20Valid
      (Audio|Components|Audio|Stop (Variables|Default|GetTrack)))
    (:Is%20Not%20Valid
      _))
  (bind _returnvalue (Audio|CreateSound2D Song 1.0 1.0 0.0 0))
  (bind _output_get (Variables|Default|SetTrack _returnvalue))
  (Audio|Components|Audio|Play _output_get 0.0))

(fn StopTrack
  (bind _track (Variables|Default|GetTrack))
  (if (Variables|Default|GetPlaying)
    (if (Utilities|IsValid _track)
      (Audio|Components|Audio|Stop _track))))

(fn LowerVolume
  (bind _track (Variables|Default|GetTrack))
  (if (Variables|Default|GetPlaying)
    (if (Utilities|IsValid _track)
      (Audio|Components|Audio|AdjustVolume _track 3.5 0.0 "Linear" :!class /Script/Engine.AudioComponent))))