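; BP_Tree is a Paper2D tree with animated leaves that can be faded out and in.
; When Activated, it waits a random sub-second delay, then plays the MoveLeaves timeline to stretch the leaves in X and offset them.
; Each timeline update also copies the main sprite's color to the leaves.
; FadeOut and FadeIn step that sprite's alpha in undelayed loops, so each completes within one frame, and toggle Invisible.
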(event EventBeginPlay
  (bind _leaves (Variables|Default|GetLeaves))
  (bind _papersprite (Variables|Default|GetPaperSprite))
  (bind _leaves_2 (Variables|Default|GetLeaves))
  (bind _returnvalue (Transformation|GetWorldScale _leaves))
  (bind _spritecolor (Variables|/Script/Paper2D.PaperSpriteComponent|GetSpriteColor _papersprite))
  (if (Variables|Default|GetActivated?)
    (Utilities|FlowControl|Delay (Math|Random|RandomFloatinRange 0.0 1.0))
    (Variables|Default|SetBaseScale (Math|Vector|MakeVector (.x _returnvalue) (.y _returnvalue) (.z _returnvalue)))
    (bind (_direction _scaleadd _worldoffset) (Timeline|MoveLeaves PlayFromStart)
      (:Update
        (Transformation|SetWorldScale3D _leaves_2 (Math|Vector|MakeVector (+ (.x (Variables|Default|GetBaseScale)) _scaleadd) (.y (Variables|Default|GetBaseScale)) (.z (Variables|Default|GetBaseScale))))
        (Transformation|AddWorldOffset _leaves_2 (Math|Vector|MakeVector _worldoffset 0.0 (* _worldoffset 0.5)) false false)
        (if (== _spritecolor (Variables|/Script/Paper2D.PaperSpriteComponent|GetSpriteColor (Variables|Default|GetLeaves)))
          _
          (else
            _))
        (Sprite|SetSpriteColor (Variables|Default|GetLeaves) _spritecolor)))))

(fn ConstructionScript)

(fn FadeOut
  (bind _papersprite (Variables|Default|GetPaperSprite))
  (bind _spritecolor (Variables|/Script/Paper2D.PaperSpriteComponent|GetSpriteColor _papersprite))
  (bind (_r _g _b _a) (Math|Color|BreakColor _spritecolor))
  (if (not (Variables|Default|GetInvisible))
    (while (> _a 0.0)
      (Sprite|SetSpriteColor _papersprite (Math|Color|MakeColor _r _g _b (+ _a -0.02))))
    (Variables|Default|SetInvisible true)))

(fn Fadein
  (bind _papersprite (Variables|Default|GetPaperSprite))
  (bind _spritecolor (Variables|/Script/Paper2D.PaperSpriteComponent|GetSpriteColor _papersprite))
  (bind (_r _g _b _a) (Math|Color|BreakColor _spritecolor))
  (if (Variables|Default|GetInvisible)
    (while (< _a 1.0)
      (Sprite|SetSpriteColor _papersprite (Math|Color|MakeColor _r _g _b (+ _a 0.02))))
    (Variables|Default|SetInvisible false)))