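; BP_AmbientChange is a trigger actor that shifts the color of a referenced light when the player overlaps it.
; Each begin overlap from any actor flips a toggle, but only Player-tagged actors then start the DarkenSky timeline, forward or in reverse according to that toggle.
; The timeline's color track drives the light component of LightRef on update.
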(event Collision|EventActorBeginOverlap
  (params (OtherActor :type Actor%20Object%20Reference))
  (Variables|Default|SetActivateDeactivate (not (Variables|Default|GetActivateDeactivate)))
  (if (Actor|ActorHasTag OtherActor "Player")
    (if (Variables|Default|GetActivateDeactivate)
      (bind _newtrack_0 (Timeline|DarkenSky PlayFromStart)
        (:Update
          (Rendering|Components|Light|SetLightColor (Variables|/Script/Engine.Light|GetLightComponent (Variables|Default|GetLightRef)) _newtrack_0 true)))
      (else
        (Timeline|DarkenSky ReverseFromEnd)))))

(event EventBeginPlay)

(fn ConstructionScript)