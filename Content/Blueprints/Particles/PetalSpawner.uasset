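; PetalSpawner is an actor that repeatedly spawns either a Petals or a Snow actor at its own transform.
; It uses its own Tick as the spawn timer by setting the tick interval to SpawnRate on BeginPlay.
; While Activated is set, each tick spawns Petals if PetalsSnow is true and Snow otherwise, then enables ticking on the new actor.
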(event EventBeginPlay
  (Actor|Tick|SetActorTickInterval (Variables|Default|GetSpawnRate)))

(event EventTick
  (params (DeltaSeconds :type Float%20%28single-precision%29))
  (bind _returnvalue (Transformation|GetActorTransform))
  (if (Variables|Default|GetActivated)
    (if (Variables|Default|GetPetals/Snow)
      (bind _returnvalue_2 (Game|SpawnActorfromClass "/Game/Blueprints/Particles/Petals.Petals_C" _returnvalue "Undefined" "MultiplyWithRoot" 0 0))
      (if (Utilities|IsValid _returnvalue_2)
        (Actor|Tick|SetActorTickEnabled _returnvalue_2 true))
      (else
        (bind _returnvalue_3 (Game|SpawnActorfromClass "/Game/Blueprints/Particles/Snow.Snow_C" _returnvalue "Undefined" "MultiplyWithRoot" 0 0))
        (if (Utilities|IsValid _returnvalue_3)
          (Actor|Tick|SetActorTickEnabled _returnvalue_3 true))))))

(fn ConstructionScript)