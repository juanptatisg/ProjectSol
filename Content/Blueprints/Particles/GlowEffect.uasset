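; GlowEffect is a particle Blueprint that makes a Paper2D sprite pulse like a glow, fading and scaling in and out.
; A random startup delay of up to a second staggers instances before a looping one-second timer flips the Growing flag.
; While Activated, each Tick adds or subtracts FadeRate on alpha and GrowRate on X and Z scale, without delta-time scaling, so pulse amplitude depends on frame rate.
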(event Custom|StartGlow
  (Variables|Default|SetGrowing (not (Variables|Default|GetGrowing))))

(event EventBeginPlay
  (Utilities|FlowControl|Delay (Math|Random|RandomFloatinRange 0.0 1.0))
  (Utilities|Time|SetTimerbyEvent (delegate Custom|StartGlow) 1.0 true))

(event EventTick
  (params (DeltaSeconds :type Float%20%28single-precision%29))
  (bind _growrate (Variables|Default|GetGrowRate))
  (bind _papersprite (Variables|Default|GetPaperSprite))
  (bind _growing (Variables|Default|GetGrowing))
  (bind _papersprite_2 (Variables|Default|GetPaperSprite))
  (bind _returnvalue (Transformation|GetWorldScale _papersprite))
  (bind _returnvalue_2 (select _growing 1.0 -1.0))
  (bind _spritecolor (Variables|/Script/Paper2D.PaperSpriteComponent|GetSpriteColor _papersprite_2))
  (bind (_x _y _z) (Class|KismetMathLibrary|BreakVector3f _returnvalue))
  (bind (_r _g _b _a) (Math|Color|BreakColor _spritecolor))
  (bind _returnvalue_3 (* _returnvalue_2 _growrate))
  (if (Variables|Default|GetActivated)
    (Sprite|SetSpriteColor _papersprite_2 (Math|Color|MakeColor _r _g _b (+ _a (* (select (Variables|Default|GetGrowing) 1.0 -1.0) (Variables|Default|GetFadeRate)))))
    (Transformation|SetWorldScale3D _papersprite (Math|Vector|MakeVector (+ _x _returnvalue_3) _y (+ _z _returnvalue_3)))))

(fn ConstructionScript)