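; PetalActivator is a trigger actor that switches a set of spawners, presumably for petal particles, on or off when the player overlaps it.
; On overlap by an actor tagged Player, it sets the Activated flag on every entry in SpawnerArray to match its TurnOn mode.
; Its own Activated flag guards the loop, so spawners are written only when that flag differs from TurnOn.
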(event EventBeginPlay)

(event Collision|EventActorBeginOverlap
  (params (OtherActor :type Actor%20Object%20Reference))
  (if (Actor|ActorHasTag OtherActor "Player")
    (if (Variables|Default|GetTurnOn)
      (if (not (Variables|Default|GetActivated))
        (for _array_element (Variables|Default|GetSpawnerArray)
          (Variables|/Game/Blueprints/Particles/PetalSpawner.PetalSpawner_C|SetActivated _array_element true))
        (Variables|Default|SetActivated true))
      (elif (Variables|Default|GetActivated)
        (for _array_element_2 (Variables|Default|GetSpawnerArray)
          (Variables|/Game/Blueprints/Particles/PetalSpawner.PetalSpawner_C|SetActivated _array_element_2 false))
        (Variables|Default|SetActivated false)))))

(fn ConstructionScript)