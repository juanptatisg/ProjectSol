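; Effect controller component that spawns hit visual effects for battler attacks.
; Custom events for energy light, combo light and combo heavy attacks each take the battler's location and spawn scaled-down effect actors at hand-tuned offsets from it.
; Delays time the spawns, so the combo events stagger several rapier hits in sequence, while the energy attack spawns one ring hit and plays a sound with slightly randomized pitch.
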(event Custom|ComboLight
  (params (BattlerLocation :type Vector))
  (Utilities|FlowControl|Delay 0.2)
  (Game|SpawnActorfromClass "/Game/Blueprints/Particles/PlayerVFX/EF_RapierHit.EF_RapierHit_C" (Math|Transform|MakeTransform (+ BattlerLocation "180.000000,70.000000,60.000000") "0, 0, 0" "0.400000,0.400000,0.400000") "Undefined" "MultiplyWithRoot" 0 0)
  (Utilities|FlowControl|Delay 0.2)
  (Game|SpawnActorfromClass "/Game/Blueprints/Particles/PlayerVFX/EF_RapierHit.EF_RapierHit_C" (Math|Transform|MakeTransform (+ BattlerLocation "160.000000,70.000000,90.000000") "0, 0, 0" "0.400000,0.400000,0.400000") "Undefined" "MultiplyWithRoot" 0 0))

(event Custom|ComboHeavy
  (params (BattlerLocation :type Vector))
  (Utilities|FlowControl|Delay 0.1)
  (Game|SpawnActorfromClass "/Game/Blueprints/Particles/PlayerVFX/EF_RapierHit.EF_RapierHit_C" (Math|Transform|MakeTransform (+ BattlerLocation "210.000000,70.000000,70.000000") "0, 0, 0" "0.400000,0.400000,0.400000") "Undefined" "MultiplyWithRoot" 0 0)
  (Utilities|FlowControl|Delay 0.1)
  (Game|SpawnActorfromClass "/Game/Blueprints/Particles/PlayerVFX/EF_RapierHit.EF_RapierHit_C" (Math|Transform|MakeTransform (+ BattlerLocation "190.000000,70.000000,90.000000") "0, 0, 0" "0.400000,0.400000,0.400000") "Undefined" "MultiplyWithRoot" 0 0)
  (Utilities|FlowControl|Delay 0.1)
  (Game|SpawnActorfromClass "/Game/Blueprints/Particles/PlayerVFX/EF_RapierHit.EF_RapierHit_C" (Math|Transform|MakeTransform (+ BattlerLocation "220.000000,70.000000,40.000000") "0, 0, 0" "0.400000,0.400000,0.400000") "Undefined" "MultiplyWithRoot" 0 0)
  (Utilities|FlowControl|Delay 0.1)
  (Game|SpawnActorfromClass "/Game/Blueprints/Particles/PlayerVFX/EF_RapierHit.EF_RapierHit_C" (Math|Transform|MakeTransform (+ BattlerLocation "210.000000,70.000000,50.000000") "0, 0, 0" "0.400000,0.400000,0.400000") "Undefined" "MultiplyWithRoot" 0 0)
  (Utilities|FlowControl|Delay 0.1)
  (Game|SpawnActorfromClass "/Game/Blueprints/Particles/PlayerVFX/EF_RapierHit.EF_RapierHit_C" (Math|Transform|MakeTransform (+ BattlerLocation "180.000000,70.000000,100.000000") "0, 0, 0" "0.400000,0.400000,0.400000") "Undefined" "MultiplyWithRoot" 0 0))

(event Custom|EnergyLight
  (params (BattlerLocation :type Vector))
  (Utilities|FlowControl|Delay 0.2)
  (Game|SpawnActorfromClass "/Game/Blueprints/Particles/PlayerVFX/EF_RingHit.EF_RingHit_C" (Math|Transform|MakeTransform (+ BattlerLocation "186.000000,70.000000,45.000000") "0, 0, 0" "0.400000,0.400000,0.400000") "Undefined" "MultiplyWithRoot" 0 0)
  (Audio|PlaySound2D "/Game/Assets/Audio/SFX/EnergyATK1.EnergyATK1" 1.0 (Math|Random|RandomFloatinRange 1.0 1.05) 0.0 0 0))