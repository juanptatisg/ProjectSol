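; PetalMovement is an actor in the particles folder that follows the player, apparently to carry a petal effect.
; BeginPlay finds actors tagged Player and stores the BP_PlayerBase reference.
; Each Tick flips a boolean and teleports the actor to the player's location plus a height offset, alternating between opposite fixed X offsets every frame.
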(event EventBeginPlay
  (bind _outactors (Actor|GetAllActorswithTag "Player"))
  (for _array_element _outactors
    (bind _asbp_player_base (Utilities|Casting|CastToBP_PlayerBase _array_element))
    (Variables|Default|SetPlayer _asbp_player_base)))

(event EventTick
  (params (DeltaSeconds :type Float%20%28single-precision%29))
  (bind _player (Variables|Default|GetPlayer))
  (bind _player_2 (Variables|Default|GetPlayer))
  (bind _returnvalue (Transformation|GetActorLocation _player))
  (bind _returnvalue_2 (Transformation|GetActorLocation _player_2))
  (bind (_x _y _z) (Class|KismetMathLibrary|BreakVector3f _returnvalue))
  (bind (_x_2 _y_2 _z_2) (Class|KismetMathLibrary|BreakVector3f _returnvalue_2))
  (bind _output_get (Variables|Default|SetVariance (not (Variables|Default|GetVariance))))
  (if _output_get
    (Transformation|SetActorLocation (Math|Vector|MakeVector (+ _x -8e+01) _y (+ _z (Variables|Default|GetHeightOffset))) false true)
    (else
      (Transformation|SetActorLocation (Math|Vector|MakeVector (+ _x_2 8e+01) _y_2 (+ _z_2 (Variables|Default|GetHeightOffset))) false true))))

(fn ConstructionScript)