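; BP_PerfectParry is a short-lived player VFX actor that shows a perfect parry as a sprite that expands and fades out.
; Each Tick grows the PaperSprite along X and Z, the sprite plane, while lowering its color alpha.
; The actor destroys itself once the alpha is nearly depleted.
; Steps are fixed per frame without delta time, so the effect's speed depends on frame rate.
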(event EventBeginPlay)

(event Collision|EventActorBeginOverlap
  (params (OtherActor :type Actor%20Object%20Reference)))

(event EventTick
  (params (DeltaSeconds :type Float%20%28single-precision%29))
  (bind _papersprite (Variables|Default|GetPaperSprite))
  (bind _papersprite_2 (Variables|Default|GetPaperSprite))
  (bind _returnvalue (Transformation|GetWorldScale _papersprite))
  (bind _spritecolor (Variables|/Script/Paper2D.PaperSpriteComponent|GetSpriteColor _papersprite_2))
  (bind (_r _g _b _a) (Math|Color|BreakColor _spritecolor))
  (bind (_x _y _z) (Math|Vector|BreakVector _returnvalue))
  (bind _returnvalue_2 (- _a 0.06))
  (Transformation|SetWorldScale3D _papersprite_2 (Math|Vector|MakeVector (+ _x 0.005) _y (+ _z 0.005)))
  (Sprite|SetSpriteColor _papersprite_2 (Math|Color|MakeColor _r _g _b _returnvalue_2))
  (if (<= _returnvalue_2 0.0)
    (Actor|DestroyActor)))

(fn ConstructionScript)