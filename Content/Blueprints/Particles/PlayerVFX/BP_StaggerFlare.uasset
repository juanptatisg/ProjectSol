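; BP_StaggerFlare is a short-lived player VFX actor that shows a sprite flare, by its name for a stagger.
; On BeginPlay its Effect timeline plays at triple speed, driving the Paper2D sprite's scale and alpha while the sprite rotates a fixed pitch step each update.
; The actor destroys itself when the timeline finishes.
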(event EventBeginPlay
  (bind _papersprite (Variables|Default|GetPaperSprite))
  (bind _spritecolor (Variables|/Script/Paper2D.PaperSpriteComponent|GetSpriteColor _papersprite))
  (bind (_r _g _b) (Math|Color|BreakColor _spritecolor))
  (Components|Timeline|SetPlayRate (Variables|Default|GetEffect) 3.0)
  (bind (_direction _scale _alpha) (Timeline|Effect PlayFromStart)
    (:Update
      (Transformation|SetWorldScale3D _papersprite (Math|Vector|MakeVector _scale _scale _scale))
      (Transformation|AddWorldRotation (Variables|Default|GetPaperSprite) (Math|Rotator|MakeRotator 0.0 2.0 0.0) false false)
      (Sprite|SetSpriteColor (Variables|Default|GetPaperSprite) (Math|Color|MakeColor _r _g _b _alpha)))
    (:Finished
      (Actor|DestroyActor))))

(fn ConstructionScript)