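; Game mode for the main menu that shows the menu widget and launches the forest level.
; BeginPlay creates UI_MainMenu, adds it to the viewport, shows the cursor and locks input to UI only.
; Tick polls a PlayPressed flag, then removes the menu, restores game-only input and opens Landscape_Forest with BP_GameModeBase as the game mode.
; A few animation and flipbook nodes are left unconnected.
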(event EventBeginPlay
  (bind _returnvalue (Game|GetPlayerController 0))
  (bind _output_get (Variables|Default|SetCharacterRef 0))
  (bind _returnvalue_2 (UserInterface|CreateWidget "/Game/Blueprints/UI/MainMenu/UI_MainMenu.UI_MainMenu_C" _output_get))
  (UserInterface|Viewport|AddtoViewport _returnvalue_2 0)
  (bind _output_get_2 (Variables|/Script/Engine.PlayerController|SetbShowMouseCursor _returnvalue true))
  (Input|SetInputModeUIOnly _returnvalue _returnvalue_2 "LockAlways" _output_get_2))

(event EventTick
  (params (DeltaSeconds :type Float%20%28single-precision%29))
  (bind _returnvalue (Game|GetPlayerController 0))
  (if (Variables|Default|GetPlayPressed)
    (Widget|RemovefromParent (Variables|Default|GetMainMenu))
    (Variables|/Script/Engine.PlayerController|SetbShowMouseCursor _returnvalue false)
    (Input|SetInputModeGameOnly _returnvalue false)
    (Game|OpenLevel(byName) "Landscape_Forest" true "?Game=/Game/Blueprints/BP_GameModeBase.BP_GameModeBase_C")))

(fn ConstructionScript)