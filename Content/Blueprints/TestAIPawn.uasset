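; Test AI pawn that moves toward the first player character.
; BeginPlay casts that character to BP_PlayerBase, stores it, waits one tick, then issues a single AI MoveTo with the player as target actor.
; Tick caches the player's location in PlayerPOS, which also feeds the move's destination.
; A failed move only prints a debug string, with no retry.
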(event Custom|FollowPlayer
  (AI|AIMoveTo self (Variables|Default|GetPlayerPOS) (Variables|Default|Getplayer) 5.0 false
    (:OnFail
      (Development|PrintString "FAILLL"))))

(event EventTick
  (params (DeltaSeconds :type Float%20%28single-precision%29))
  (Variables|Default|SetPlayerPOS (Transformation|GetActorLocation (Variables|Default|Getplayer))))

(event EventBeginPlay
  (bind _asbp_player_base (Utilities|Casting|CastToBP_PlayerBase (Game|GetPlayerCharacter 0)))
  (Variables|Default|Setplayer _asbp_player_base)
  (Utilities|FlowControl|DelayUntilNextTick)
  (CallFunction|FollowPlayer))

(fn ConstructionScript)