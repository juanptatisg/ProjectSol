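; BP_LuciaDoor is a vine door with a skeletal mesh that opens when the player walks into its trigger box.
; It loops a closed idle from BeginPlay, then on the first player overlap plays the opening animation and sets IsDoorOpen, with no path to close again.
; While open, Tick calls PlayAnimation with the open idle every frame, overriding the opening animation.
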(event OnComponentBeginOverlap(Box)
  (params (OverlappedComponent :type Primitive%20Component%20Object%20Reference) (OtherActor :type Actor%20Object%20Reference) (OtherComp :type Primitive%20Component%20Object%20Reference) (OtherBodyIndex :type Integer) (bFromSweep :type Boolean) (SweepResult :type Hit%20Result%20Structure%20%28by%20ref%29))
  (if (not (Variables|Default|GetIsDoorOpen))
    (if (== OtherActor (Game|Player|GetPlayerPawn 0))
      (Components|Animation|PlayAnimation (Variables|Default|GetSkeletalMesh) "/Game/Assets/Meshes/Trees/DoorVines/AS_LuciaDoorVines_VineOpen_Anim.AS_LuciaDoorVines_VineOpen_Anim" false)
      (bind _output_get (Variables|Default|SetIsDoorOpen true)))))

(event EventBeginPlay
  (Variables|Default|SetIsDoorOpen false)
  (Components|Animation|PlayAnimation (Variables|Default|GetSkeletalMesh) "/Game/Assets/Meshes/Trees/DoorVines/AS_LuciaDoorVines_VineIdleClosed_Anim.AS_LuciaDoorVines_VineIdleClosed_Anim" (not (Variables|Default|GetIsDoorOpen))))

(event EventTick
  (params (DeltaSeconds :type Float%20%28single-precision%29))
  (if (stale OnComponentBeginOverlap(Box) _output_get)
    (Components|Animation|PlayAnimation (Variables|Default|GetSkeletalMesh) "/Game/Assets/Meshes/Trees/DoorVines/AS_LuciaDoorVines_VineIdleOpen_Anim.AS_LuciaDoorVines_VineIdleOpen_Anim" (stale OnComponentBeginOverlap(Box) _output_get))))

(fn ConstructionScript)